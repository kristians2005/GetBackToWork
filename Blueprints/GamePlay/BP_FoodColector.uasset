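; Food collector actor that detects base item actors inside its box volume, reporting or clearing them.
; Getfood gathers the data asset of each overlapping item into a list and returns it.
; DeleteAllFood destroys overlapping items except those in BP_BoundBox's ImportantObjects, then activates a Niagara effect.
; GiveFoodDataToTarget is a stub that always returns false.
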(event `/Game/Blueprints/GamePlay/BPI_FoodReciver.DeleteAllFood`
  (bind _output_get (set `self.Overlapingactors` (`PrimitiveComponent.GetOverlappingActors` (`self.Box`) "/Game/Blueprints/CookingItems/A_BP_BaseItem_Master.A_BP_BaseItem_Master_C")))
  (for _array_element _output_get
    (bind _returnvalue (`GameplayStatics.GetActorOfClass` "/Game/Blueprints/Actors/BoundBox/BP_BoundBox.BP_BoundBox_C"))
    (bind _ref (message `/Game/Blueprints/BPI/BPI_BaseItem.GetBaseItemSelfRef` _array_element))
    (if (not (`KismetArrayLibrary.Array_Contains` (`/Game/Blueprints/Actors/BoundBox/BP_BoundBox.ImportantObjects` _returnvalue) _ref))
      (`self.K2_DestroyActor` _array_element)))
  (`ActorComponent.Activate` (`self.NewNiagaraSystem`) true))

(fn `Getfood`
  (returns (NewParam :type "Array of /Game/Blueprints/DataAssets/Items/DA_Item Object Reference"))
  (locals (L_DAITEMS :type "Array of /Game/Blueprints/DataAssets/Items/DA_Item Object Reference"))
  (for _array_element (`PrimitiveComponent.GetOverlappingActors` (`self.Box`) "/Game/Blueprints/CookingItems/A_BP_BaseItem_Master.A_BP_BaseItem_Master_C")
    (bind _getdaiten (message `/Game/Blueprints/BPI/BPI_BaseItem.GetDAItem` _array_element))
    (`KismetArrayLibrary.Array_Add` (`local.L_DAITEMS`) _getdaiten))
  (return (`local.L_DAITEMS`)))

(fn `GiveFoodDataToTarget`
  (params (Data :type "/Game/Blueprints/DataAssets/Items/DA_Item Object Reference") (AmountJustOne :type Boolean :default false))
  (returns (`Success?` :type Boolean))
  (return false))

(fn `UserConstructionScript`)