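; BP_TV is an in-world television that shows the game mode's message widget on its screen component.
; On BeginPlay it fetches the message widget from the game mode and assigns it to the WScreen widget component, retrying every 0.2 seconds until it is valid.
; Its other functions, covering widget access, food and recipe tag receipt and tool checks, are empty stubs.
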(event `self.ReceiveBeginPlay`
  (bind _widgetref (message `/Game/Blueprints/BPI/BPI_GameMode.GetWidget` (`GameplayStatics.GetGameMode`) :!label _label))
  (`/Engine/EditorBlueprintResources/StandardMacros.IsValid` _widgetref
    (:`Is Valid`
      (`WidgetComponent.SetWidget` (`self.W_Screen`) _widgetref))
    (:`Is Not Valid`
      (`KismetSystemLibrary.Delay` 0.2)
      (goto _label))))

(event `self.ReceiveTick`
  (params (DeltaSeconds :type "Float (single-precision)")))

(fn `GetWidget`
  (returns (widgetRef :type "/Game/Blueprints/GamePlay/W_Receipt Object Reference"))
  (return null))

(fn `HandleReciveFood`
  (returns (FoodOrder :type "Array of Actor Object Reference"))
  (return))

(fn `IsTool_GM`
  (returns (IsTool :type Boolean))
  (return false))

(fn `Recive item recipe Tags`
  (returns (Tags :type "GameplayTagContainer Structure"))
  (return))

(fn `UserConstructionScript`)