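; BP_ReceiptPrinter is a printer actor that feeds out a paper receipt for the current order.
; SpawnNewReceipt stores the order data and prints, while the printer button reprints the stored order, ignoring requests during an active print.
; Printing spawns BP_ReceipePaper with physics off, then a timeline slides it from PaperPrinterArrow to VerpTo, stopping early if the paper is grabbed.
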(event `SpawnPaper`
  (bind _returnvalue (`SceneComponent.K2_GetComponentToWorld` (`self.PaperPrinterArrow`)))
  (bind _returnvalue_location (`KismetMathLibrary.BreakTransform` (`SceneComponent.K2_GetComponentToWorld` (`self.verpTo`))))
  (bind _returnvalue_location_2 (`KismetMathLibrary.BreakTransform` (`SceneComponent.K2_GetComponentToWorld` (`self.PaperPrinterArrow`))))
  (if (`KismetArrayLibrary.Array_IsNotEmpty` (`self.Current Order Data`))
    (if (not (`self.IsPrintingRn`))
      (bind _returnvalue_2 (`|SpawnActorFromClass` "/Game/Blueprints/CookingItems/BP_ReceipePaper.BP_ReceipePaper_C" (`KismetMathLibrary.MakeTransform` (`KismetMathLibrary.MakeVector` (.x (.location _returnvalue)) (.y (.location _returnvalue)) (.z (.location _returnvalue))) (.rotation _returnvalue) (.scale _returnvalue)) "Undefined" "MultiplyWithRoot" null (`self.Current Order Data`) null))
      (bind _output_get (set `self.ReceiptRef` _returnvalue_2))
      (`/Game/Blueprints/BPI/BPI_BaseItem.SetSimulatePhisics?` _output_get false)
      (set `self.IsPrintingRn` true)
      (bind (_direction _alpha) (`Timeline|Timeline` :!via `PlayFromStart` :!label _label)
        (:`Update`
          (if (`/Game/Blueprints/CookingItems/A_BP_BaseItem_Master.IsRN_Grabed` (`self.ReceiptRef`))
            (set `self.IsPrintingRn` false)
            (goto _label :!via `Stop`)
            (else
              (`SceneComponent.K2_SetWorldLocation` (`/Game/Blueprints/CookingItems/A_BP_BaseItem_Master.BaseItem` (`self.ReceiptRef`)) (`KismetMathLibrary.VLerp` _returnvalue_location_2 _returnvalue_location _alpha) false true))))
        (:`Finished`
          (set `self.IsPrintingRn` false))))))

(event `SpawnNewReceipt`
  (params (`Order data` :type "Array of /Game/Blueprints/Structs/ST_Order Structure"))
  (set `self.Current Order Data` `Order data`)
  (`self.SpawnPaper`))

(event `/Game/Blueprints/BPI/BPI_Buttons.Printer-Btn`
  (`self.SpawnPaper`))

(fn `UserConstructionScript`)