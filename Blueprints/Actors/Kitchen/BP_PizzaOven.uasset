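; BP_PizzaOven is a kitchen oven actor that tells items when they enter or leave its cooking space.
; The OvenInside overlap component sends interface messages to overlapping actors, passing a fixed enum value on entry and signalling removal on exit.
; GetWhatOvenCanCook returns a fixed enum value, while the smoke, base mesh and ingredient mesh functions are empty or return false.
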(event `self.Oven inside.OnComponentBeginOverlap`
  (params (OverlappedComponent :type "PrimitiveComponent Object Reference") (OtherActor :type "Actor Object Reference") (OtherComp :type "PrimitiveComponent Object Reference") (OtherBodyIndex :type Integer) (bFromSweep :type Boolean) (SweepResult :type "HitResult Structure (by ref)"))
  (`/Engine/EditorBlueprintResources/StandardMacros.IsValid` OtherActor
    (:`Is Valid`
      (message `/Game/Blueprints/BPI/BPI_FoodCooking.ItemPlacedOnCookingOven` OtherActor "NewEnumerator2"))))

(event `self.Oven inside.OnComponentEndOverlap`
  (params (OverlappedComponent :type "PrimitiveComponent Object Reference") (OtherActor :type "Actor Object Reference") (OtherComp :type "PrimitiveComponent Object Reference") (OtherBodyIndex :type Integer))
  (`/Engine/EditorBlueprintResources/StandardMacros.IsValid` OtherActor
    (:`Is Valid`
      (message `/Game/Blueprints/BPI/BPI_FoodCooking.ItemTakenOffCookingOven` OtherActor))))

(fn `ActivateSmoke`
  (returns (`Success?` :type Boolean))
  (return false))

(fn `GetBaseItemMesh`
  (returns (`Mesh Component` :type "MeshComponent Object Reference"))
  (return null))

(fn `GetFoodIngredientMeshes`
  (returns (`Scene component` :type "Array of SceneComponent Object Reference") (`success?` :type Boolean))
  (return _ false))

(fn `GetWhatOvenCanCook`
  (returns (`WhatOvenType?` :type "/Game/Blueprints/Enums/E_WhatOvenCanCook Enum"))
  (return "NewEnumerator0"))

(fn `UserConstructionScript`)