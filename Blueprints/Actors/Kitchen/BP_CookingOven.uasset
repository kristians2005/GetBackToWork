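; BP_CookingOven is a kitchen oven actor that cooks food items placed inside its Box trigger.
; Overlapping actors implementing BPI_FoodCooking are notified when placed on or taken off, and entering starts a looping timer that stops once no base items remain.
; That timer toggles cooking feedback: a faded ItemCooking sound and a Timeline-driven glow on the dynamic cooker material.
; BPCOven handles placement requests, while items spawn at the player's hit point.
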(event `self.ReceiveBeginPlay`
  (`/Game/Blueprints/BPC/BPC_Oven.Init` (`self.BPC_Oven`) self)
  (bind _returnvalue (`PrimitiveComponent.CreateDynamicMaterialInstance` (`self.StaticMesh`) 0 "/Game/Materials/Textures/Kitchen/Coocker/M_Cooker.M_Cooker" "None"))
  (set `self.M_CookerRef` _returnvalue))

(event `self.Box.OnComponentBeginOverlap`
  (params (OverlappedComponent :type "PrimitiveComponent Object Reference") (OtherActor :type "Actor Object Reference") (OtherComp :type "PrimitiveComponent Object Reference") (OtherBodyIndex :type Integer) (bFromSweep :type Boolean) (SweepResult :type "HitResult Structure (by ref)"))
  (`/Engine/EditorBlueprintResources/StandardMacros.IsValid` OtherActor
    (:`Is Valid`
      (if (`KismetSystemLibrary.DoesImplementInterface` OtherActor "/Game/Blueprints/BPI/BPI_FoodCooking.BPI_FoodCooking_C")
        (message `/Game/Blueprints/BPI/BPI_FoodCooking.ItemPlacedOnCookingOven` OtherActor "NewEnumerator1")
        (`KismetSystemLibrary.K2_SetTimer` null "PlayCookingAnim" 0.5 true true)))))

(event `self.Box.OnComponentEndOverlap`
  (params (OverlappedComponent :type "PrimitiveComponent Object Reference") (OtherActor :type "Actor Object Reference") (OtherComp :type "PrimitiveComponent Object Reference") (OtherBodyIndex :type Integer))
  (`/Engine/EditorBlueprintResources/StandardMacros.IsValid` OtherActor
    (:`Is Valid`
      (message `/Game/Blueprints/BPI/BPI_FoodCooking.ItemTakenOffCookingOven` OtherActor))))

(event `PlayCookingAnim`
  (if (not (`self.isAnimActive?`))
    (`self.HottnesAnimOn`)
    (set `self.isAnimActive?` true))
  (if (<= (`KismetArrayLibrary.Array_Length` (`PrimitiveComponent.GetOverlappingActors` (`self.Box`) "/Game/Blueprints/CookingItems/A_BP_BaseItem_Master.A_BP_BaseItem_Master_C")) 0)
    (`self.HottnesAnimOff`)
    (set `self.isAnimActive?` false)
    (`KismetSystemLibrary.K2_ClearTimer` null "PlayCookingAnim")))

(event `HottnesAnimOn`
  (bind _itemcooking (`self.ItemCooking`))
  (`AudioParameterControllerInterface.SetBoolParameter` _itemcooking "CookingItem" true)
  (`AudioComponent.FadeIn` _itemcooking 0.5 1.0 0.0 "Linear")
  (bind (_direction _alpha) (`Timeline|Timeline` :!via `PlayFromStart` :!label _label)
    (:`Update`
      (`MaterialInstanceDynamic.SetScalarParameterValue` (`self.M_CookerRef`) "Light strenght" (`KismetMathLibrary.Lerp` 0.0 0.6 _alpha)))))

(event `HottnesAnimOff`
  (bind _itemcooking (`self.ItemCooking`))
  (`AudioParameterControllerInterface.SetBoolParameter` _itemcooking "CookingItem" true)
  (`AudioComponent.FadeOut` _itemcooking 0.5 0.0 "Linear")
  (goto _label :!via `Reverse`))

(event `/Game/Blueprints/BPI/BPI_OvenFoodReciver.SpawnItemOnOven`
  (params (ObjectClass :type "/Game/Blueprints/CookingItems/A_BP_BaseItem_Master Class Reference"))
  (bind _hitpoint (message `/Game/Blueprints/BPI/BPI_Interaction.GetHitPoint` (`GameplayStatics.GetPlayerCharacter` 0)))
  (`|SpawnActorFromClass` ObjectClass (`KismetMathLibrary.MakeTransform` _hitpoint) "Undefined" "MultiplyWithRoot" null true null))

(fn `ActivateSmoke`
  (returns (`Success?` :type Boolean))
  (return false))

(fn `FlatMode_Interaction`
  (returns (BaseItemMasterRef :type "/Game/Blueprints/CookingItems/A_BP_BaseItem_Master Object Reference") (InteractionType :type "/Game/Blueprints/Enums/E_InteractionTypes Enum") (Actor :type "Actor Object Reference"))
  (return null "NewEnumerator2" self))

(fn `GetBaseItemMesh`
  (returns (`Mesh Component` :type "MeshComponent Object Reference"))
  (return null))

(fn `GetFoodIngredientMeshes`
  (returns (`Scene component` :type "Array of SceneComponent Object Reference") (`success?` :type Boolean))
  (return _ false))

(fn `GetHitPoint`
  (returns (HitPoint :type "Vector Structure"))
  (return (0.0 0.0 0.0)))

(fn `GetWhatOvenCanCook`
  (returns (`WhatOvenType?` :type "/Game/Blueprints/Enums/E_WhatOvenCanCook Enum"))
  (return "NewEnumerator0"))

(fn `TryPlaceFoodOnOven`
  (params (DA_Item :type "/Game/Blueprints/DataAssets/Items/DA_Item Object Reference"))
  (returns (Success :type Boolean))
  (bind _success_ (`/Game/Blueprints/BPC/BPC_Oven.PlaceItemToOven` (`self.BPC_Oven`) DA_Item))
  (return _success_))

(fn `UserConstructionScript`)