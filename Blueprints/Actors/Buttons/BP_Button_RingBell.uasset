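; BP_Button_RingBell is a bell button actor that notifies a target actor when pressed.
; BTNPressed sends PressedMessage to TargetActor and plays the Bell sound at the static mesh's location.
; GetWidget, HandleReciveFood and the recipe-tag function are empty stubs, and IsToolGM returns false.
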(event `self.ReceiveBeginPlay`
  (`parent.ReceiveBeginPlay`))

(event `self.BTN_Pressed`
  (message `/Game/Blueprints/BPI/BPI_Buttons.Pressed` (`self.TargetActor`))
  (`GameplayStatics.PlaySoundAtLocation` "/Game/Sound/SoundQues/Bell.Bell" (`SceneComponent.K2_GetComponentLocation` (`self.StaticMesh`)) (struct) 1.0 1.0 0.0 null null null null))

(fn `GetWidget`
  (returns (widgetRef :type "/Game/Blueprints/GamePlay/W_Receipt Object Reference"))
  (return null))

(fn `HandleReciveFood`
  (returns (FoodOrder :type "Array of Actor Object Reference"))
  (return))

(fn `IsTool_GM`
  (returns (IsTool :type Boolean))
  (return false))

(fn `Recive item recipe Tags`
  (returns (Tags :type "GameplayTagContainer Structure"))
  (return))

(fn `UserConstructionScript`
  (`parent.UserConstructionScript`))