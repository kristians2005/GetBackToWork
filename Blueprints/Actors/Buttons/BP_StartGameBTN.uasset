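; BP_StartGameBTN is a button actor that launches the start-game intro cutscene.
; Its BTNPressed event passes through a DoOnce, finds the BP_StartGameIntro actor with GetActorOfClass and calls PlayCutsceen on it.
; The DoOnce keeps repeated presses from replaying the intro, while BeginPlay and construction only call the parent.
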(event `self.ReceiveBeginPlay`
  (`parent.ReceiveBeginPlay`))

(event `self.BTN_Pressed`
  (`/Engine/EditorBlueprintResources/StandardMacros.DoOnce` false
    (:`Completed`
      (bind _returnvalue (`GameplayStatics.GetActorOfClass` "/Game/Blueprints/Actors/BP_StartGameIntro.BP_StartGameIntro_C"))
      (`/Game/Blueprints/Actors/BP_StartGameIntro.PlayCutsceen` _returnvalue))))

(fn `UserConstructionScript`
  (`parent.UserConstructionScript`))