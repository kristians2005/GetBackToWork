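; Numbered keypad button actor for a microwave, holding an integer Value that the construction script shows on its Text component.
; An init event stores the owning microwave's reference, and BTNPressed passes the button's Value to that microwave through MicrowaveCodeSendMessage.
; The widget, food-receiving, recipe-tag and tool-check functions are empty stubs, with IsToolGM returning false.
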(event `self.ReceiveBeginPlay`
  (`parent.ReceiveBeginPlay`))

(event `/Game/Blueprints/BPI/BPI_Buttons.Microwave-btns-INIT`
  (params (microwaveRef :type "Actor Object Reference"))
  (set `self.Microwave Ref` microwaveRef))

(event `self.BTN_Pressed`
  (message `/Game/Blueprints/BPI/BPI_Buttons.Microwave code send` (`self.Microwave Ref`) (`self.Value`)))

(fn `GetWidget`
  (returns (widgetRef :type "/Game/Blueprints/GamePlay/W_Receipt Object Reference"))
  (return null))

(fn `HandleReciveFood`
  (returns (FoodOrder :type "Array of Actor Object Reference"))
  (return))

(fn `IsTool_GM`
  (returns (IsTool :type Boolean))
  (return false))

(fn `Recive item recipe Tags`
  (returns (Tags :type "GameplayTagContainer Structure"))
  (return))

(fn `UserConstructionScript`
  (`parent.UserConstructionScript`)
  (`TextRenderComponent.K2_SetText` (`self.Text`) (`KismetTextLibrary.Conv_IntToText` (`self.Value`))))