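; Button actor for the heating machine that, when pressed, calls CallHeatingMachineMessage on its target actor.
; BeginPlay creates a dynamic glow material, which the oven status event flashes green briefly before turning black and the clear-all event blacks out.
; The construction script writes the placeholder label text.
; The general food machine status event and CallFoodMachine are empty.
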(event `self.ReceiveBeginPlay`
  (`parent.ReceiveBeginPlay`)
  (bind _returnvalue (`PrimitiveComponent.CreateDynamicMaterialInstance` (`self.Glow`) 0 "/Game/Blueprints/Actors/Buttons/M_FoodMachineGlow.M_FoodMachineGlow" "None"))
  (set `self.M_GlowRef` _returnvalue))

(event `self.BTN_Pressed`
  (message `/Game/Blueprints/BPI/BPI_Buttons.CallHeatingMachine` (`self.TargetActor`)))

(event `self.UpdateAllFoodMachineBTN_Status`
  (params (Success :type Boolean)))

(event `/Game/Blueprints/BPI/BPI_Buttons.UpdateOvenBTNStatus`
  (`MaterialInstanceDynamic.SetVectorParameterValue` (`self.M_GlowRef`) "color" (struct :`R` 0.436549 :`G` 1.0 :`B` 0.435382 :`A` 1.0))
  (`KismetSystemLibrary.Delay` 0.5)
  (`MaterialInstanceDynamic.SetVectorParameterValue` (`self.M_GlowRef`) "color" (struct :`A` 1.0)))

(event `self.FoodMachineClearAllGlow`
  (`MaterialInstanceDynamic.SetVectorParameterValue` (`self.M_GlowRef`) "color" (struct :`A` 1.0)))

(fn `CallFoodMachine`
  (params (DA_Item :type "/Game/Blueprints/DataAssets/Items/DA_Item Object Reference") (BtnType :type "/Game/Blueprints/Actors/FoodMachine/E_FoodM_BTN_Type Enum" :default "NewEnumerator0")))

(fn `UserConstructionScript`
  (`parent.UserConstructionScript`)
  (`TextRenderComponent.K2_SetText` (`self.PlaceHolder`) (`self.Placeholder_text`)))