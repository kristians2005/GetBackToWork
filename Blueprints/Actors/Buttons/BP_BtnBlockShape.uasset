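; BP_BtnBlockShape is a button actor that relays presses to a target machine, apparently adapted from microwave and coffee machine buttons.
; A microwave button init event stores the passed reference as the target.
; On press, it sends a coffee machine button message carrying its CoffeeType to the target actor.
; Its widget, food, tool and recipe-tag functions are empty stubs, with the tool check returning false.
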(event `self.ReceiveBeginPlay`
  (`parent.ReceiveBeginPlay`))

(event `self.Microwave-btns-INIT`
  (params (microwaveRef :type "Actor Object Reference"))
  (set `self.Target` microwaveRef))

(event `self.BTN_Pressed`
  (message `/Game/Blueprints/BPI/BPI_Buttons.Coffee-Machine-Btn` (`self.TargetActor`) (`self.Coffee Type`)))

(fn `GetWidget`
  (returns (widgetRef :type "/Game/Blueprints/GamePlay/W_Receipt Object Reference"))
  (return null))

(fn `HandleReciveFood`
  (returns (FoodOrder :type "Array of Actor Object Reference"))
  (return))

(fn `IsTool_GM`
  (returns (IsTool :type Boolean))
  (return false))

(fn `Recive item recipe Tags`
  (returns (Tags :type "GameplayTagContainer Structure"))
  (return))

(fn `UserConstructionScript`
  (`parent.UserConstructionScript`))