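; BP_Restart is a button actor that restarts play by opening M_FinalLevel when pressed.
; Its BTNPressed event runs once, calls FadeScreenMessage on the player character with a short fade and a long hold, waits a second, then loads the level.
; BeginPlay and construction only call the parent versions, while overlap and tick are disabled.
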(event `self.ReceiveBeginPlay`
  (`parent.ReceiveBeginPlay`))

(event `self.BTN_Pressed`
  (`/Engine/EditorBlueprintResources/StandardMacros.DoOnce` false
    (:`Completed`
      (message `/Game/Blueprints/BPI/BPI_Interaction.FadeScreen` (`GameplayStatics.GetPlayerCharacter` 0) false false false 0.07 222.0)
      (`KismetSystemLibrary.Delay` 1.0)
      (`GameplayStatics.OpenLevelBySoftObjectPtr` "/Game/Maps/M_FinalLevel.M_FinalLevel"))))

(fn `UserConstructionScript`
  (`parent.UserConstructionScript`))