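; Music player actor that controls background music and ambient sound, using tracks mostly from FNAF soundtracks.
; AmbianceSounds fades in lamp ambiance on BeginPlay, and FadeAmbiance fades it in or out on demand.
; ChangeMusic switches MusicPlayer by enum with per-track fade-ins, skipping Venta Black if already set.
; FadeOutMusic applies per-track fade-out times to whatever is playing, with no action for People Ambiance.
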(event `self.ReceiveBeginPlay`
  (`AudioComponent.SetSound` (`self.AmbianceSounds`) "/Game/Sound/LampAmbiance/LampAmbiance.LampAmbiance")
  (`AudioComponent.FadeIn` (`self.AmbianceSounds`) 3.0 1.0 0.0 "Linear"))

(event `/Game/Blueprints/BPI/BPI_Music.ChangeMusic`
  (params (Music :type "/Game/Blueprints/DataAssets/RushHour/E_Song Enum" :default "NewEnumerator0"))
  (bind _sound (`AudioComponent.Sound` (`self.MusicPlayer`)))
  (switch `/Game/Blueprints/DataAssets/RushHour/E_Song` Music
    (:`NewEnumerator1`
      (`AudioComponent.SetSound` (`self.MusicPlayer`) "/Game/Sound/Music/Tragedy_and_Comedy__Hesitation__-_FNAF__Secret_of_the_Mimic_OST.Tragedy_and_Comedy__Hesitation__-_FNAF__Secret_of_the_Mimic_OST")
      (`AudioComponent.FadeIn` (`self.MusicPlayer`) 1.0 1.0 0.0 "Linear"))
    (:`NewEnumerator2`
      (`AudioComponent.SetSound` (`self.MusicPlayer`) "/Game/Sound/Music/FNAF_Security_Breach_OST__Supernova_Journey__Unused_.FNAF_Security_Breach_OST__Supernova_Journey__Unused_")
      (`AudioComponent.FadeIn` (`self.MusicPlayer`) 0.2 1.0 0.0 "Linear"))
    (:`NewEnumerator3`
      (if (not (== _sound "/Game/Sound/Music/FNAF_SISTER_LOCATION_-_Venta_Black__HQ_.FNAF_SISTER_LOCATION_-_Venta_Black__HQ_"))
        (`/Game/Blueprints/BPFL/BPFL_GlobalFunctions.Debug - Print string` (`KismetSystemLibrary.GetDisplayName` _sound))
        (`AudioComponent.SetSound` (`self.MusicPlayer`) "/Game/Sound/Music/FNAF_SISTER_LOCATION_-_Venta_Black__HQ_.FNAF_SISTER_LOCATION_-_Venta_Black__HQ_")
        (`AudioComponent.FadeIn` (`self.MusicPlayer`) 2.0 1.0 0.0 "Linear")))
    (:`NewEnumerator4`
      (`AudioComponent.SetSound` (`self.MusicPlayer`) "/Game/Sound/Music/Help_Wanted_2_OST__Phantogeusia__Sleep_No_More_Remix_.Help_Wanted_2_OST__Phantogeusia__Sleep_No_More_Remix_")
      (`AudioComponent.FadeIn` (`self.MusicPlayer`) 1.0 1.0 0.0 "Linear"))
    (:`NewEnumerator5`
      (`AudioComponent.SetSound` (`self.MusicPlayer`) "/Game/Sound/Music/FNAF_Pizzeria_Simulator_OST_18_-_Ambient_People.FNAF_Pizzeria_Simulator_OST_18_-_Ambient_People")
      (`AudioComponent.FadeIn` (`self.MusicPlayer`) 3.0 1.0 0.0 "Linear"))))

(event `/Game/Blueprints/BPI/BPI_Music.FadeAmbiance`
  (params (`FadeIn : FadeOut` :type Boolean) (Duration :type "Float (double-precision)"))
  (bind _ambiancesounds (`self.AmbianceSounds`))
  (if `FadeIn : FadeOut`
    (`AudioComponent.FadeIn` _ambiancesounds Duration 1.0 0.0 "Linear")
    (else
      (`AudioComponent.FadeOut` _ambiancesounds Duration 0.0 "Linear"))))

(event `/Game/Blueprints/BPI/BPI_Music.FadeOutMusic`
  (params (Music :type "/Game/Blueprints/DataAssets/RushHour/E_Song Enum" :default "NewEnumerator0"))
  (bind _musicplayer (`self.MusicPlayer`))
  (switch `/Game/Blueprints/DataAssets/RushHour/E_Song` Music
    (:`NewEnumerator1`
      (`AudioComponent.FadeOut` _musicplayer 3.0 0.0 "Linear"))
    (:`NewEnumerator2`
      (`AudioComponent.FadeOut` _musicplayer 5.0 0.0 "Linear"))
    (:`NewEnumerator3`
      (`AudioComponent.FadeOut` _musicplayer 3.0 0.0 "Linear"))
    (:`NewEnumerator4`
      (`AudioComponent.FadeOut` _musicplayer 5.0 0.0 "Linear"))))

(fn `UserConstructionScript`)