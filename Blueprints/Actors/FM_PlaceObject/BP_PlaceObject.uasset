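; Placement spot actor that snaps items of allowed classes to its PlaceLocation, supporting both flatmode and VR play.
; In flatmode, hovering briefly flashes a Niagara effect for matching items, and interacting has the VR pawn put the held item down there.
; In VR, overlapping the box releases the item from the hand and snaps it in, occupying the spot until that item exits OuterLayer.
; Placed items are notified on VR placement and removal.
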(event `self.ReceiveBeginPlay`
  (if (`/Game/Blueprints/BPFL/BPFL_GlobalFunctions.IsFlatmode`)
    (bind _asvrpawn (cast `/Game/Game_BP/VRTemplate/Blueprints/VRPawn` (`GameplayStatics.GetPlayerPawn` 0)))
    (set `self.PlayerRef` _asvrpawn)))

(event `/Game/Blueprints/BPI/BPI_Interaction.Hover_Object-snap`
  (params (BP_BaseItem :type "/Game/Blueprints/CookingItems/A_BP_BaseItem_Master Object Reference"))
  (if (`/Game/Blueprints/BPFL/BPFL_GlobalFunctions.IsFlatmode`)
    (if (`SceneComponent.IsVisible` (`self.Niagara`))
      _
      (elif (not (not (`self.Does object match with allowed objects` BP_BaseItem)))
        (`SceneComponent.SetVisibility` (`self.Niagara`) true false)
        (`KismetSystemLibrary.Delay` 0.1)
        (`SceneComponent.SetVisibility` (`self.Niagara`) false false)))))

(event `/Game/Blueprints/BPI/BPI_Interaction.FM_Interact`
  (params (CurrentHoldItem :type "/Game/Blueprints/CookingItems/A_BP_BaseItem_Master Object Reference"))
  (bind _placelocation (`self.PlaceLocation`))
  (bind _placelocation_2 (`self.PlaceLocation`))
  (if (`/Game/Blueprints/BPFL/BPFL_GlobalFunctions.IsFlatmode`)
    (set `self.Current Held Object` CurrentHoldItem)
    (if (`KismetArrayLibrary.Array_IsEmpty` (`self.AllowedObjects`))
      _
      (elif (not (not (`self.Does object match with allowed objects` (`self.Current Held Object`))))
        (`/Game/Game_BP/VRTemplate/Blueprints/VRPawn.FM_PlaceItemDown` (`self.PlayerRef`) (`/Game/Blueprints/CookingItems/A_BP_BaseItem_Master.BaseItem` (`self.Current Held Object`)) (`SceneComponent.K2_GetComponentLocation` _placelocation_2) false false (`SceneComponent.K2_GetComponentRotation` _placelocation_2) true)
        (`/Game/Blueprints/BPI/BPI_BaseItem.MoveObjectToTheSpot_OrSMTH` (`self.Current Held Object`) (`SceneComponent.K2_GetComponentLocation` _placelocation) (`SceneComponent.K2_GetComponentRotation` _placelocation) false)))))

(event `self.PlaceCollisionBox.OnComponentBeginOverlap`
  (params (OverlappedComponent :type "PrimitiveComponent Object Reference") (OtherActor :type "Actor Object Reference") (OtherComp :type "PrimitiveComponent Object Reference") (OtherBodyIndex :type Integer) (bFromSweep :type Boolean) (SweepResult :type "HitResult Structure (by ref)"))
  (bind _placelocation (`self.PlaceLocation`))
  (if (`KismetArrayLibrary.Array_Contains` (`ActorComponent.ComponentTags` OtherComp) "BaseItemCol")
    (if (`self.CanPlaceDown?`)
      (if (not (`/Game/Blueprints/BPFL/BPFL_GlobalFunctions.IsFlatmode`))
        (`/Engine/EditorBlueprintResources/StandardMacros.IsValid` (`self.PlacedItemRef`)
          (:`Is Not Valid`
            (bind _ref (message `/Game/Blueprints/BPI/BPI_BaseItem.GetBaseItemSelfRef` OtherActor))
            (if (`self.Does object match with allowed objects` _ref)
              (set `self.CanPlaceDown?` false)
              (set `self.PlacedItemRef` OtherActor)
              (bind _grabcomponent (`/Game/Blueprints/CookingItems/A_BP_BaseItem_Master.GrabComponent` _ref))
              (if (`/Game/Game_BP/VRTemplate/Blueprints/GrabComponent.bIsHeld` _grabcomponent)
                (message `/Game/Blueprints/BPI/BPI_Interaction.VR_ReleaseFromHand` (`GameplayStatics.GetPlayerCharacter` 0) (`/Game/Game_BP/VRTemplate/Blueprints/GrabComponent.GetHeldByHand` _grabcomponent)))
              (`/Game/Blueprints/BPI/BPI_BaseItem.MoveObjectToTheSpot_OrSMTH` _ref (`SceneComponent.K2_GetComponentLocation` _placelocation) (`SceneComponent.K2_GetComponentRotation` _placelocation) (`self.VRMode_ShouldHavePhysicsWhenPlaced`))
              (message `/Game/Blueprints/BPI/BPI_BaseItem.ItemPlacedDown` _ref))))))))

(event `self.OuterLayer.OnComponentEndOverlap`
  (params (OverlappedComponent :type "PrimitiveComponent Object Reference") (OtherActor :type "Actor Object Reference") (OtherComp :type "PrimitiveComponent Object Reference") (OtherBodyIndex :type Integer))
  (if (`KismetArrayLibrary.Array_Contains` (`ActorComponent.ComponentTags` OtherComp) "BaseItemCol")
    (if (not (`/Game/Blueprints/BPFL/BPFL_GlobalFunctions.IsFlatmode`))
      (`/Engine/EditorBlueprintResources/StandardMacros.IsValid` (`self.PlacedItemRef`)
        (:`Is Valid`
          (if (== (`self.PlacedItemRef`) OtherActor)
            (set `self.CanPlaceDown?` true)
            (message `/Game/Blueprints/BPI/BPI_BaseItem.ItemTakenAway` (`self.PlacedItemRef`))
            (set `self.PlacedItemRef` null)))))))

(fn `Does object match with allowed objects`
  (params (Object :type "Object Object Reference"))
  (returns (`Does match?` :type Boolean))
  (for _array_element (`self.AllowedObjects`)
    (if (== _array_element (`GameplayStatics.GetObjectClass` Object))
      (return true)))
  (return false))

(fn `FlatMode_Interaction`
  (returns (BaseItemMasterRef :type "/Game/Blueprints/CookingItems/A_BP_BaseItem_Master Object Reference") (InteractionType :type "/Game/Blueprints/Enums/E_InteractionTypes Enum") (Actor :type "Actor Object Reference"))
  (return null "NewEnumerator2" self))

(fn `GetHitPoint`
  (returns (HitPoint :type "Vector Structure"))
  (return (0.0 0.0 0.0)))

(fn `GetVRPawnRef`
  (returns (NewParam :type "/Game/Game_BP/VRTemplate/Blueprints/VRPawn Object Reference"))
  (return null))

(fn `UserConstructionScript`)