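; BP_Clock is a clock actor that displays the game time held by BP_Brain as hours and minutes.
; On BeginPlay it caches the first BP_Brain found in the level.
; Tick runs through a 0.6-second Delay, which throttles how often the Time text is rebuilt from the brain's Hours and Minutes in H:M format.
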(event `self.ReceiveBeginPlay`
  (bind _outactors (`GameplayStatics.GetAllActorsOfClass` "/Game/Game_BP/BP_Brain.BP_Brain_C"))
  (set `self.BrainRef` (`|GetArrayItem` _outactors)))

(event `self.ReceiveTick`
  (params (DeltaSeconds :type "Float (single-precision)"))
  (bind (_days _hours _minutes) (`KismetMathLibrary.BreakTimespan2` (`/Game/Game_BP/BP_Brain.Time` (`self.BrainRef`))))
  (`KismetSystemLibrary.Delay` 0.6)
  (`TextRenderComponent.K2_SetText` (`self.Time`) (`|FormatText` "{H}:{M}" (`KismetTextLibrary.Conv_IntToText` _hours false true 2 2) (`KismetTextLibrary.Conv_IntToText` _minutes false true 2 2))))

(fn `UserConstructionScript`)