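; BP_Trashcan is a trash can actor that destroys items dropped into its Box trigger.
; On overlap, it only handles actors derived from A_BP_BaseItem_Master and requires a valid BoundRef.
; It asks BoundRef through a MoveImportantItemsBack message whether to rescue the item, and destroys it only when that returns false.
; Its own GetBoundBoxLeftObject, GetSelf, IsThisBaseItem and MoveImportantItemsBack functions are stubs returning empty or false.
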(event `self.Box.OnComponentBeginOverlap`
  (params (OverlappedComponent :type "PrimitiveComponent Object Reference") (OtherActor :type "Actor Object Reference") (OtherComp :type "PrimitiveComponent Object Reference") (OtherBodyIndex :type Integer) (bFromSweep :type Boolean) (SweepResult :type "HitResult Structure (by ref)"))
  (bind _boundref (`self.BoundRef`))
  (`/Engine/EditorBlueprintResources/StandardMacros.IsValid` OtherActor
    (:`Is Valid`
      (if (`KismetMathLibrary.ClassIsChildOf` (`GameplayStatics.GetObjectClass` OtherActor) "/Game/Blueprints/CookingItems/A_BP_BaseItem_Master.A_BP_BaseItem_Master_C")
        (`/Engine/EditorBlueprintResources/StandardMacros.IsValid` _boundref
          (:`Is Valid`
            (bind _success (message `/Game/Blueprints/BPI/BPI_BaseItem.MoveImportantItemsBack` _boundref OtherActor))
            (if (not _success)
              (`self.K2_DestroyActor` OtherActor))))))))

(fn `GetBoundBoxLeftObject`
  (returns (object :type "/Game/Blueprints/CookingItems/A_BP_BaseItem_Master Object Reference"))
  (return null))

(fn `GetSelf`
  (returns (BP_BaseItem :type "/Game/Blueprints/CookingItems/A_BP_BaseItem_Master Object Reference"))
  (return null))

(fn `IsThisBaseItem?`
  (returns (Success :type Boolean))
  (return false))

(fn `MoveImportantItemsBack`
  (params (actor :type "Actor Object Reference"))
  (returns (success :type Boolean))
  (return false))

(fn `UserConstructionScript`)