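; BP_SimpleCarDriveBy is an ambient car that repeatedly drives along its spline at random intervals.
; After a random delay it resets to the actor root, becomes visible and gets a random color from ColorArr through a dynamic material instance.
; A slowed timeline moves it along the spline, smoothing yaw toward the path direction with RInterpTo.
; When the run finishes, it hides and schedules the next pass.
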(event `self.ReceiveBeginPlay`
  (bind _returnvalue (`PrimitiveComponent.CreateDynamicMaterialInstance` (`self.StaticMesh`) 0 "/Game/Assets/Props/Car/CarBase.CarBase" "None"))
  (set `self.MateralRef` _returnvalue)
  (`SceneComponent.SetVisibility` (`self.StaticMesh`) false false)
  (`self.PickRandomTImeToSpawnCar`))

(event `PickRandomTImeToSpawnCar`
  (`KismetSystemLibrary.Delay` (`KismetMathLibrary.RandomFloatInRange` 10.0 30.0))
  (`self.DriveCar`))

(event `DriveCar`
  (bind _scene (`self.Scene`))
  (bind _colorarr (`self.ColorArr`))
  (bind _spline (`self.Spline`))
  (`SceneComponent.K2_SetWorldLocationAndRotation` :`self` (`self.Scene`) :`NewLocation` (`SceneComponent.K2_GetComponentLocation` (`self.DefaultSceneRoot`)))
  (`SceneComponent.SetVisibility` (`self.StaticMesh`) true false)
  (`MaterialInstanceDynamic.SetVectorParameterValue` (`self.MateralRef`) "Color" (`|GetArrayItem` _colorarr (`KismetMathLibrary.RandomIntegerInRange` 0 (- (`KismetArrayLibrary.Array_Length` _colorarr) 1))))
  (`KismetSystemLibrary.Delay` 1.0)
  (`TimelineComponent.SetPlayRate` (`self.Timeline`) 0.2)
  (bind (_direction _alpha) (`Timeline|Timeline` :!via `PlayFromStart`)
    (:`Update`
      (bind _returnvalue (`KismetMathLibrary.Lerp` 0.0 (`SplineComponent.GetSplineLength` _spline) _alpha))
      (bind (_returnvalue_roll _returnvalue_pitch _returnvalue_yaw) (`KismetMathLibrary.BreakRotator` (`KismetMathLibrary.MakeRotFromX` (`SplineComponent.GetDirectionAtDistanceAlongSpline` _spline _returnvalue "World"))))
      (`SceneComponent.K2_SetWorldLocationAndRotation` _scene (`SplineComponent.GetLocationAtDistanceAlongSpline` (`self.Spline`) _returnvalue "World") (`KismetMathLibrary.RInterpTo` (`SceneComponent.K2_GetComponentRotation` _scene) (`KismetMathLibrary.MakeRotator` 0.0 0.0 _returnvalue_yaw) (`GameplayStatics.GetWorldDeltaSeconds`) 6.0) false false))
    (:`Finished`
      (`KismetSystemLibrary.Delay` 1.0)
      (`SceneComponent.SetVisibility` (`self.StaticMesh`) false false)
      (`self.PickRandomTImeToSpawnCar`))))

(fn `UserConstructionScript`)