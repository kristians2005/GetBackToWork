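; Retrieve point actor with a shaft door that toggles between open and closed through Close/OpenShaftDoor.
; A single Timeline slides the door down by DoorGap from its BeginPlay position to close and plays in reverse to open, with a sound at each start.
; CanCloseDoor blocks new toggles until the movement finishes.
; CallFoodMachine is a stub that returns false.
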(event `self.ReceiveBeginPlay`
  (set `self.OpenDoorLocation` (`SceneComponent.RelativeLocation` (`self.Door`))))

(event `/Game/Blueprints/BPI/BPI_Buttons.Close/Open_ShaftDoor`
  (if (`self.CanCloseDoor?`)
    (if (`self.IsDoorOpen?`)
      (`self.CloseDoor`)
      (else
        (`self.OpenDoor`)))))

(event `CloseDoor`
  (bind (_opendoorlocation_x _opendoorlocation_y _opendoorlocation_z) (`KismetMathLibrary.BreakVector` (`self.OpenDoorLocation`)))
  (set `self.IsDoorOpen?` false)
  (set `self.CanCloseDoor?` false)
  (`GameplayStatics.PlaySoundAtLocation` "/Game/Sound/SFX2/LiftDoor/SC_DoorOpen.SC_DoorOpen" (`SceneComponent.K2_GetComponentLocation` (`self.Door`)) (struct) 1.0 1.0 0.0 null null null null)
  (bind (_direction _alpha) (`Timeline|Timeline` :!via `PlayFromStart` :!label _label)
    (:`Update`
      (`SceneComponent.K2_SetRelativeLocation` (`self.Door`) (`KismetMathLibrary.MakeVector` _opendoorlocation_x _opendoorlocation_y (`KismetMathLibrary.Lerp` _opendoorlocation_z (- _opendoorlocation_z (`self.DoorGap`)) _alpha)) false true))
    (:`Finished`
      (set `self.CanCloseDoor?` true))))

(event `OpenDoor`
  (set `self.IsDoorOpen?` true)
  (set `self.CanCloseDoor?` false)
  (`GameplayStatics.PlaySoundAtLocation` "/Game/Sound/SFX2/LiftDoor/SC_DoorClose.SC_DoorClose" (`SceneComponent.K2_GetComponentLocation` (`self.Door`)) (struct) 1.0 1.0 0.0 null null null null)
  (goto _label :!via `ReverseFromEnd`))

(fn `CallFoodMachine`
  (params (DA_Item :type "/Game/Blueprints/DataAssets/Items/DA_Item Object Reference") (BtnType :type "/Game/Blueprints/Actors/FoodMachine/E_FoodM_BTN_Type Enum" :default "NewEnumerator0"))
  (returns (`success?` :type Boolean))
  (return false))

(fn `UserConstructionScript`)