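; BP_HeatingOven is an oven actor that cooks pizza dough and turns pancake dough bowls into pancakes.
; CallHeatingMachine checks the first overlapping actor of each type in its Box and sends it a cook or conversion message.
; Each success updates the BP_HeatingMachineBTN found in the level and plays the oven sound.
; It also stores a switch angle it never reads, and CallFoodMachine only returns false.
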(event `/Game/Blueprints/BPI/BPI_Buttons.CallHeatingMachine`
  (bind _output (`|GetArrayItem` (`PrimitiveComponent.GetOverlappingActors` (`self.Box`) "/Game/Blueprints/CookingItems/Kitchen/Pot/BP_FoodBowl_PancakeDough.BP_FoodBowl_PancakeDough_C")))
  (bind _output_2 (`|GetArrayItem` (`PrimitiveComponent.GetOverlappingActors` (`self.Box`) "/Game/Blueprints/CookingItems/Pizza/BP_PizzaDough.BP_PizzaDough_C")))
  (`|ExecutionSequence`
    (:`then_0`
      (`/Engine/EditorBlueprintResources/StandardMacros.IsValid` _output_2
        (:`Is Valid`
          (bind _success_ (message `/Game/Blueprints/BPI/BPI_BaseItem.CanBeCooked?` _output_2))
          (if _success_
            (message `/Game/Blueprints/BPI/BPI_FoodCooking.SetItemCookedState` _output_2 "NewEnumerator1")
            (bind _returnvalue (`GameplayStatics.GetActorOfClass` "/Game/Blueprints/Actors/Buttons/BP_HeatingMachineBTN.BP_HeatingMachineBTN_C"))
            (`/Game/Blueprints/BPI/BPI_Buttons.UpdateOvenBTNStatus` _returnvalue)
            (`GameplayStatics.PlaySoundAtLocation` "/Game/Sound/SFX2/Oven/Oven.Oven" (`SceneComponent.K2_GetComponentLocation` (`self.Box`)) (struct) 1.0 1.0 0.0 null null null null)))))
    (:`then_1`
      (`/Engine/EditorBlueprintResources/StandardMacros.IsValid` _output
        (:`Is Valid`
          (bind _success (message `/Game/Blueprints/BPI/BPI_BaseItem.ChangeToPankcakes` _output))
          (if _success
            (bind _returnvalue_2 (`GameplayStatics.GetActorOfClass` "/Game/Blueprints/Actors/Buttons/BP_HeatingMachineBTN.BP_HeatingMachineBTN_C"))
            (`/Game/Blueprints/BPI/BPI_Buttons.UpdateOvenBTNStatus` _returnvalue_2)
            (`GameplayStatics.PlaySoundAtLocation` "/Game/Sound/SFX2/Oven/Oven.Oven" (`SceneComponent.K2_GetComponentLocation` (`self.Box`)) (struct) 1.0 1.0 0.0 null null null null)))))))

(event `/Game/Blueprints/BPI/BPI_Buttons.GetSwitchCurrentRollAngleIDFK`
  (params (CurrnetAngle :type "Float (double-precision)"))
  (set `self.Currnet Angle` CurrnetAngle))

(fn `CallFoodMachine`
  (params (DA_Item :type "/Game/Blueprints/DataAssets/Items/DA_Item Object Reference") (BtnType :type "/Game/Blueprints/Actors/FoodMachine/E_FoodM_BTN_Type Enum" :default "NewEnumerator0"))
  (returns (`success?` :type Boolean))
  (return false))

(fn `UserConstructionScript`)