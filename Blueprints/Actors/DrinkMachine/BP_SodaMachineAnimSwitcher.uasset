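; BP_SodaMachineAnimSwitcher is a soda machine actor that animates its material by stepping through three states in a loop.
; After a short delay on BeginPlay, it creates a dynamic instance of M_SodaMachine on the UpdatedSodaMachineV1 component.
; A looping one-second timer then calls PlayAnim, which cycles a counter and writes it to the material's Value scalar parameter.
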(event `self.ReceiveBeginPlay`
  (`KismetSystemLibrary.Delay` 1.0)
  (bind _returnvalue (`PrimitiveComponent.CreateDynamicMaterialInstance` (`self.UpdatedSodaMachineV1`) 0 "/Game/Materials/Textures/Kitchen/SodaMachine/M_SodaMachine.M_SodaMachine" "None"))
  (set `self.NewVar` _returnvalue)
  (`KismetSystemLibrary.K2_SetTimer` null "PlayAnim" 1.0 true true))

(event `PlayAnim`
  (bind _returnvalue (+ (`self.Val`) 1))
  (if (< _returnvalue 3)
    (set `self.Val` _returnvalue)
    (else
      (set `self.Val` 0)))
  (`MaterialInstanceDynamic.SetScalarParameterValue` (`self.NewVar`) "Value" (`KismetMathLibrary.Conv_IntToDouble` (`self.Val`))))

(fn `UserConstructionScript`)