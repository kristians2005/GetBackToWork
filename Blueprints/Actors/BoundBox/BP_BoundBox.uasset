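; BP_BoundBox is a boundary volume that sends important items back to their spawn place when they leave it.
; On BoundCollisionBox end overlap, unless that component is tagged "ignor", it resolves the actor via GetBoundBoxLeftObjectMessage and matches it against ImportantObjects.
; MoveImportantItemsBack runs the same recovery on demand, passing true instead of false.
; MoveBackObject, a sweep-teleport helper, is uncalled here; other item query functions are empty stubs.
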(event `self.BoundCollisionBox.OnComponentEndOverlap`
  (params (OverlappedComponent :type "PrimitiveComponent Object Reference") (OtherActor :type "Actor Object Reference") (OtherComp :type "PrimitiveComponent Object Reference") (OtherBodyIndex :type Integer))
  (`/Engine/EditorBlueprintResources/StandardMacros.IsValid` OtherActor
    (:`Is Valid`
      (if (not (`KismetArrayLibrary.Array_Contains` (`ActorComponent.ComponentTags` OverlappedComponent) "ignor"))
        (bind (_item _success) (`self.CheckImportantObjects` OtherActor))
        (if _success
          (`/Game/Blueprints/CookingItems/A_BP_BaseItem_Master.MoveObjectBackToSpawnPlace` _item false))))))

(fn `CanBeCooked?`
  (returns (`Success?` :type Boolean))
  (return false))

(fn `ChangeToPankcakes`
  (returns (Success :type Boolean))
  (return false))

(fn `CheckImportantObjects`
  (params (actor :type "Object Object Reference"))
  (returns (Item :type "/Game/Blueprints/CookingItems/A_BP_BaseItem_Master Object Reference") (success :type Boolean))
  (bind _object (message `/Game/Blueprints/BPI/BPI_BaseItem.GetBoundBoxLeftObject` actor))
  (for _array_element (`self.ImportantObjects`)
    (if (== _array_element _object)
      (return _array_element true)))
  (return null false))

(fn `GetBaseItemSelfRef`
  (returns (Ref :type "/Game/Blueprints/CookingItems/A_BP_BaseItem_Master Object Reference"))
  (return null))

(fn `GetBoundBoxLeftObject`
  (returns (object :type "/Game/Blueprints/CookingItems/A_BP_BaseItem_Master Object Reference"))
  (return null))

(fn `GetDAItem`
  (returns (GetDAIten :type "/Game/Blueprints/DataAssets/Items/DA_Item Object Reference"))
  (return null))

(fn `GetSelf`
  (returns (BP_BaseItem :type "/Game/Blueprints/CookingItems/A_BP_BaseItem_Master Object Reference"))
  (return null))

(fn `IsThisBaseItem?`
  (returns (Success :type Boolean))
  (return false))

(fn `MoveBackObject`
  (params (Item :type "/Game/Blueprints/CookingItems/A_BP_BaseItem_Master Object Reference"))
  (bind (_itemspawntransform_location _itemspawntransform_rotation) (`KismetMathLibrary.BreakTransform` (`/Game/Blueprints/CookingItems/A_BP_BaseItem_Master.ItemSpawnTransform` Item)))
  (`/Engine/EditorBlueprintResources/StandardMacros.IsValid` Item
    (:`Is Valid`
      (`/Game/Blueprints/BPFL/BPFL_GlobalFunctions.Debug - Print string` (`KismetStringLibrary.Conv_VectorToString` _itemspawntransform_location))
      (`SceneComponent.K2_SetWorldLocationAndRotation` (`/Game/Blueprints/CookingItems/A_BP_BaseItem_Master.BaseItem` Item) _itemspawntransform_location _itemspawntransform_rotation true true))))

(fn `MoveImportantItemsBack`
  (params (actor :type "Actor Object Reference"))
  (returns (success :type Boolean))
  (bind (_item _success) (`self.CheckImportantObjects` actor))
  (if _success
    (`/Game/Blueprints/CookingItems/A_BP_BaseItem_Master.MoveObjectBackToSpawnPlace` _item true)
    (return true)
    (else
      (return false))))

(fn `UserConstructionScript`)