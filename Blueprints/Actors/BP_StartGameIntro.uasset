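; Cutscene actor for the game-start intro, which ends by loading M_FinalLevel.
; PlayCutsceen hides the listed lights, then two chained timelines ramp the menu music's pitch and volume up and drag the pitch down.
; A spotlight switches on with a flashlight sound, three skeletal meshes play in staggered order, and the player's screen fades before the level opens.
; BeginPlay is empty, and leftover music and camera-move style nodes are unconnected.
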(event `self.ReceiveBeginPlay`)

(event `PlayCutsceen`
  (for _array_element (`self.Ligts`)
    (`SceneComponent.SetVisibility` (`Light.LightComponent` _array_element) false false))
  (bind (_direction _asd) (`Timeline|Timeline` :!via `PlayFromStart`)
    (:`Update`
      (bind _returnvalue (`GameplayStatics.GetActorOfClass` "/Game/Blueprints/Actors/BP_MenuMapMusicPlayer.BP_MenuMapMusicPlayer_C"))
      (bind _audio (`/Game/Blueprints/Actors/BP_MenuMapMusicPlayer.Audio` _returnvalue))
      (bind _returnvalue_2 (`KismetMathLibrary.Lerp` 1.0 2.0 _asd))
      (`AudioComponent.SetPitchMultiplier` _audio _returnvalue_2)
      (`AudioComponent.SetVolumeMultiplier` _audio _returnvalue_2))
    (:`Finished`
      (bind (_direction_2 _asd_2) (`Timeline|Timeline_0` :!via `PlayFromStart`)
        (:`Update`
          (bind _returnvalue_3 (`GameplayStatics.GetActorOfClass` "/Game/Blueprints/Actors/BP_MenuMapMusicPlayer.BP_MenuMapMusicPlayer_C"))
          (`AudioComponent.SetPitchMultiplier` (`/Game/Blueprints/Actors/BP_MenuMapMusicPlayer.Audio` _returnvalue_3) (`KismetMathLibrary.Lerp` 2.0 0.125 _asd_2)))
        (:`Finished`
          (`KismetSystemLibrary.Delay` 1.3)
          (`SceneComponent.SetVisibility` (`self.SpotLight`) true false)
          (`GameplayStatics.PlaySound2D` "/Game/Sound/SFX2/Flashlight/sfx_flashlight_off.sfx_flashlight_off" 2.0 1.0 0.0 null null)
          (`KismetSystemLibrary.Delay` 1.0)
          (`SkeletalMeshComponent.Play` (`self.SkeletalMesh1`) false)
          (`KismetSystemLibrary.Delay` 0.2)
          (`SkeletalMeshComponent.Play` (`self.SkeletalMesh2`) false)
          (`KismetSystemLibrary.Delay` 0.1)
          (`SkeletalMeshComponent.Play` (`self.SkeletalMesh`) false)
          (`KismetSystemLibrary.Delay` 2.0)
          (message `/Game/Blueprints/BPI/BPI_Interaction.FadeScreen` (`GameplayStatics.GetPlayerCharacter` 0) false false false 0.08 20.0)
          (`KismetSystemLibrary.Delay` 3.0)
          (`GameplayStatics.OpenLevelBySoftObjectPtr` "/Game/Maps/M_FinalLevel.M_FinalLevel"))))))

(fn `UserConstructionScript`)