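; BP_SouceStand is a food-source actor, apparently a sauce stand, that supplies its food data asset to callers and gives audio feedback when used with a tool.
; Outside flat mode, a BPI_Tool actor overlapping its Box plays the gulp-style SC_Gup sound.
; In flat mode, FMInteract plays the same sound when the held item is a tool.
; GetFoodDA always succeeds, returning DAItem, and GetHitPoint returns a zero vector.
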(event `self.Box.OnComponentBeginOverlap`
  (params (OverlappedComponent :type "PrimitiveComponent Object Reference") (OtherActor :type "Actor Object Reference") (OtherComp :type "PrimitiveComponent Object Reference") (OtherBodyIndex :type Integer) (bFromSweep :type Boolean) (SweepResult :type "HitResult Structure (by ref)"))
  (`/Engine/EditorBlueprintResources/StandardMacros.IsValid` OtherActor
    (:`Is Valid`
      (if (and (`KismetSystemLibrary.DoesImplementInterface` OtherActor "/Game/Blueprints/BPI/BPI_Tool.BPI_Tool_C") (not (`/Game/Blueprints/BPFL/BPFL_GlobalFunctions.IsFlatmode`)))
        (`GameplayStatics.PlaySoundAtLocation` "/Game/Sound/SoundQues/SC_Gup.SC_Gup" (`self.K2_GetActorLocation`) (struct) 1.0 1.0 0.0 null null null null)))))

(event `/Game/Blueprints/BPI/BPI_Interaction.FM_Interact`
  (params (CurrentHoldItem :type "/Game/Blueprints/CookingItems/A_BP_BaseItem_Master Object Reference"))
  (if (`KismetSystemLibrary.DoesImplementInterface` CurrentHoldItem "/Game/Blueprints/BPI/BPI_Tool.BPI_Tool_C")
    (`GameplayStatics.PlaySoundAtLocation` "/Game/Sound/SoundQues/SC_Gup.SC_Gup" (`self.K2_GetActorLocation`) (struct) 1.0 1.0 0.0 null null null null)))

(fn `FlatMode_Interaction`
  (returns (BaseItemMasterRef :type "/Game/Blueprints/CookingItems/A_BP_BaseItem_Master Object Reference") (InteractionType :type "/Game/Blueprints/Enums/E_InteractionTypes Enum") (Actor :type "Actor Object Reference"))
  (return null "NewEnumerator2" self))

(fn `GetFoodDA`
  (returns (Data :type "/Game/Blueprints/DataAssets/Items/DA_Item Object Reference") (success :type Boolean) (`AmountJustOne?` :type Boolean))
  (return (`self.DA_Item`) true false))

(fn `GetHitPoint`
  (returns (HitPoint :type "Vector Structure"))
  (return (0.0 0.0 0.0)))

(fn `UserConstructionScript`)