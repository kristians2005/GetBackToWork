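; BP_FoodMachine is a crafting machine that turns ingredients entered via buttons into food actors.
; CallFoodMachine forwards presses while CanClick is true, collecting unique items until Enter triggers FindRecipe, an order-independent match against AllRecipes.
; A match spawns the output at the Arrow; either result plays a sound and broadcasts status through BPI_FoodMachine.
; After a one-second lockout, ClearAll empties the input and resets button glows.
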(event `FoodMachineBTN`
  (params (Item :type "/Game/Blueprints/DataAssets/Items/DA_Item Object Reference") (btnType :type "/Game/Blueprints/Actors/FoodMachine/E_FoodM_BTN_Type Enum" :default "NewEnumerator0"))
  (bind (_returnvalue_location _returnvalue_rotation) (`KismetMathLibrary.BreakTransform` (`SceneComponent.K2_GetComponentToWorld` (`self.Arrow`))))
  (switch `/Game/Blueprints/Actors/FoodMachine/E_FoodM_BTN_Type` btnType
    (:`NewEnumerator0`
      ; Katru reizi kad poga ir nospiesta. DataAsset tiek saglabāts mainīgā
      (`KismetArrayLibrary.Array_AddUnique` (`self.InputedRecipes`) Item))
    (:`NewEnumerator1`
      (set `self.CanClick?` false)
      ; Comment
      (bind (_foundoutputitem _success_) (`self.FindRecipe`))
      (if _success_
        (`|SpawnActorFromClass` _foundoutputitem (`KismetMathLibrary.MakeTransform` _returnvalue_location _returnvalue_rotation) "Undefined" "MultiplyWithRoot" null true null)
        (`GameplayStatics.PlaySoundAtLocation` "/Game/Sound/SoundQues/FoodMachineSuccess.FoodMachineSuccess" (`SceneComponent.K2_GetComponentLocation` (`self.Arrow`)) (struct) 1.0 1.0 0.0 null null null null)
        (bind _outactors (`GameplayStatics.GetAllActorsWithInterface` "/Game/Blueprints/Actors/Buttons/BPI_FoodMachine.BPI_FoodMachine_C"))
        (for _array_element _outactors
          (message `/Game/Blueprints/BPI/BPI_Buttons.UpdateAllFoodMachineBTN_Status` _array_element true))
        (`KismetSystemLibrary.Delay` 1.0)
        (`self.ClearAll`)
        (set `self.CanClick?` true)
        (else
          (`GameplayStatics.PlaySoundAtLocation` "/Game/Sound/SoundQues/ui_notification_negative.ui_notification_negative" (`SceneComponent.K2_GetComponentLocation` (`self.Arrow`)) (struct) 1.0 1.0 0.0 null null null null)
          (bind _outactors_2 (`GameplayStatics.GetAllActorsWithInterface` "/Game/Blueprints/Actors/Buttons/BPI_FoodMachine.BPI_FoodMachine_C"))
          (for _array_element_2 _outactors_2
            (message `/Game/Blueprints/BPI/BPI_Buttons.UpdateAllFoodMachineBTN_Status` _array_element_2 false))
          (`KismetSystemLibrary.Delay` 1.0)
          (`self.ClearAll`)
          (set `self.CanClick?` true))))))

(fn `CallFoodMachine`
  (params (DA_Item :type "/Game/Blueprints/DataAssets/Items/DA_Item Object Reference") (BtnType :type "/Game/Blueprints/Actors/FoodMachine/E_FoodM_BTN_Type Enum" :default "NewEnumerator0"))
  (returns (`success?` :type Boolean))
  (if (`self.CanClick?`)
    (`self.FoodMachineBTN` DA_Item BtnType)
    (return true)
    (else
      (return false))))

(fn `ClearAll`
  (`KismetArrayLibrary.Array_Clear` (`self.InputedRecipes`))
  (bind _outactors (`GameplayStatics.GetAllActorsWithInterface` "/Game/Blueprints/Actors/Buttons/BPI_FoodMachine.BPI_FoodMachine_C"))
  (for _array_element _outactors
    (message `/Game/Blueprints/BPI/BPI_Buttons.FoodMachineClearAllGlow` _array_element)))

(fn `FindRecipe`
  (returns (FoundOutputItem :type "/Game/Blueprints/CookingItems/A_BP_BaseItem_Master Class Reference") (`success?` :type Boolean))
  (locals (Found :type Integer))
  (for _array_element (`self.AllRecipes`)
    (bind _recipe (`/Game/Blueprints/Actors/FoodMachine/DA_FoodMachineRecipes.Recipe` _array_element))
    (if (== (`KismetArrayLibrary.Array_Length` (`self.InputedRecipes`)) (`KismetArrayLibrary.Array_Length` _recipe))
      (set `local.Found` 0)
      (for _array_element_2 (`self.InputedRecipes`)
        (if (`KismetArrayLibrary.Array_Contains` _recipe _array_element_2)
          (set `local.Found` (+ (`local.Found`) 1))))
      (if (== (`local.Found`) (`KismetArrayLibrary.Array_Length` (`self.InputedRecipes`)))
        (return (`/Game/Blueprints/Actors/FoodMachine/DA_FoodMachineRecipes.Output` _array_element) true))))
  (return null false))

(fn `UserConstructionScript`)