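; Construction-script tube builder that lays a chosen mesh along a spline as a chain of non-colliding spline mesh segments.
; When Visibility is on, segments are spaced by SectionLenght, which comes from actor X scale unless AllowScaling is set.
; GetStartPos and GetEndPos sample local positions and tangents, clamping tangents to section length.
; The MustBeFullLenghtMeshes branch only sets a loop index and creates no meshes.
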(fn `GetEndPos`
  (params (Index :type Integer))
  (returns (Pos :type "Vector Structure") (Tan :type "Vector Structure"))
  (bind _spline (`self.Spline`))
  (bind _returnvalue (* (+ Index 1) (`self.SectionLenght`)))
  (return (`SplineComponent.GetLocationAtDistanceAlongSpline` _spline _returnvalue "Local") (`KismetMathLibrary.ClampVectorSize` (`SplineComponent.GetTangentAtDistanceAlongSpline` _spline _returnvalue "Local") 0.0 (`self.SectionLenght`))))

(fn `GetStartPos`
  (params (Index :type Integer))
  (returns (Pos :type "Vector Structure") (Tan :type "Vector Structure"))
  (bind _spline (`self.Spline`))
  (bind _returnvalue (* Index (`self.SectionLenght`)))
  (return (`SplineComponent.GetLocationAtDistanceAlongSpline` _spline _returnvalue "Local") (`KismetMathLibrary.ClampVectorSize` (`SplineComponent.GetTangentAtDistanceAlongSpline` _spline _returnvalue "Local") 0.0 (`self.SectionLenght`))))

(fn `UserConstructionScript`
  (locals (LoopIndex :type Integer))
  (bind _returnvalue_x (`KismetMathLibrary.BreakVector` (`self.GetActorScale3D`)))
  (if (`self.Visibility`)
    (if (not (`self.AllowScaling`))
      (set `self.SectionLenght` (* _returnvalue_x 100.0)))
    (if (`self.MustBeFullLenghtMeshes`)
      (for _index (range 1)
        (set `local.LoopIndex` _index))
      (else
        (for _index_2 (range (+ (`KismetMathLibrary.FTrunc` (/ (`SplineComponent.GetSplineLength` (`self.Spline`)) (`self.SectionLenght`))) 1))
          (set `local.LoopIndex` _index_2)
          (bind _returnvalue (`AddComponent|NODE_AddSplineMeshComponent-0`))
          (`StaticMeshComponent.SetStaticMesh` _returnvalue (`self.SplineMesh`))
          (`SplineMeshComponent.SetForwardAxis` _returnvalue "X" true)
          (bind (_pos _tan) (`self.GetStartPos` (`local.LoopIndex`)))
          (bind (_pos_2 _tan_2) (`self.GetEndPos` (`local.LoopIndex`)))
          (`SplineMeshComponent.SetStartAndEnd` _returnvalue _pos _tan _pos_2 _tan_2 true)
          (`PrimitiveComponent.SetCollisionEnabled` _returnvalue "NoCollision"))))))