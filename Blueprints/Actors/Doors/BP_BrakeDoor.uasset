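; BP_BrakeDoor is a door actor that slides vertically between its starting height and an EndPoint component.
; BeginPlay caches the Door's relative Z, and a timeline alpha lerps it to the EndPoint's Z on Closedoor.
; Opendoor reverses the same timeline from its end.
; The construction script sets the Door's initial height from NewLocationZ, and nothing inside this Blueprint calls the open or close events.
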(event `self.ReceiveBeginPlay`
  (bind (_relativelocation_x _relativelocation_y _relativelocation_z) (`KismetMathLibrary.BreakVector` (`SceneComponent.RelativeLocation` (`self.door`))))
  (set `self.Relative Location Z` _relativelocation_z))

(event `Close door`
  (bind _door (`self.door`))
  (bind (_relativelocation_x _relativelocation_y _relativelocation_z) (`KismetMathLibrary.BreakVector` (`SceneComponent.RelativeLocation` (`self.EndPoint`))))
  (bind (_relativelocation_x_2 _relativelocation_y_2) (`KismetMathLibrary.BreakVector` (`SceneComponent.RelativeLocation` _door)))
  (bind (_direction _alpha) (`Timeline|Timeline` :!via `PlayFromStart` :!label _label)
    (:`Update`
      (`SceneComponent.K2_SetRelativeLocation` _door (`KismetMathLibrary.MakeVector` _relativelocation_x_2 _relativelocation_y_2 (`KismetMathLibrary.Lerp` (`self.Relative Location Z`) _relativelocation_z _alpha)) false false))))

(event `Open door`
  (goto _label :!via `ReverseFromEnd`))

(fn `UserConstructionScript`
  (bind _door (`self.door`))
  (bind (_relativelocation_x _relativelocation_y) (`KismetMathLibrary.BreakVector` (`SceneComponent.RelativeLocation` _door)))
  (`SceneComponent.K2_SetRelativeLocation` _door (`KismetMathLibrary.MakeVector` _relativelocation_x _relativelocation_y (`self.New Location Z`)) false false))