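; BP_FreezerDoor is a freezer door actor that slides open and closed when a flat-mode interaction triggers it.
; BeginPlay caches the closed location, and FMInteract toggles between that and a Y offset of MoveAmount using an eased MoveComponentTo over FMOpeningTime.
; An IsAnimationPlaying flag blocks re-triggering during the move.
; FlatModeInteraction returns the interaction type and the door itself.
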(event `self.ReceiveBeginPlay`
  (set `self.StartLoaction` (`SceneComponent.RelativeLocation` (`self.Door`))))

(event `/Game/Blueprints/BPI/BPI_Interaction.FM_Interact`
  (params (CurrentHoldItem :type "/Game/Blueprints/CookingItems/A_BP_BaseItem_Master Object Reference"))
  (bind _door (`self.Door`))
  (bind (_relativelocation_x _relativelocation_y _relativelocation_z) (`KismetMathLibrary.BreakVector` (`SceneComponent.RelativeLocation` _door)))
  (if (`self.IsAnimationPlaying?`)
    _
    (elif (`self.IsOpen`)
      (set `self.IsAnimationPlaying?` true)
      (`KismetSystemLibrary.MoveComponentTo` (`self.Door`) (`self.StartLoaction`) (struct) true true (`self.FM_OpeningTime`))
      (set `self.IsOpen` false)
      (set `self.IsAnimationPlaying?` false)
      (else
        (set `self.IsAnimationPlaying?` true)
        (`KismetSystemLibrary.MoveComponentTo` _door (`KismetMathLibrary.MakeVector` _relativelocation_x (+ _relativelocation_y (`self.MoveAmount`)) _relativelocation_z) (struct) true true (`self.FM_OpeningTime`))
        (set `self.IsOpen` true)
        (set `self.IsAnimationPlaying?` false)))))

(fn `FlatMode_Interaction`
  (returns (BaseItemMasterRef :type "/Game/Blueprints/CookingItems/A_BP_BaseItem_Master Object Reference") (InteractionType :type "/Game/Blueprints/Enums/E_InteractionTypes Enum") (Actor :type "Actor Object Reference"))
  (return null "NewEnumerator2" self))

(fn `UserConstructionScript`)