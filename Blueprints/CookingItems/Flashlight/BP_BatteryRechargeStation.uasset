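; BP_BatteryRechargeStation is a recharge zone for flashlight batteries.
; Its Box overlap begin and end events send start and end recharge messages to overlapping actors that implement BPI_FlashLight, leaving the charging logic to those actors.
; Both events skip the message when the overlapped component, the station's own Box, carries the "ignor" tag.
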(event `self.Box.OnComponentBeginOverlap`
  (params (OverlappedComponent :type "PrimitiveComponent Object Reference") (OtherActor :type "Actor Object Reference") (OtherComp :type "PrimitiveComponent Object Reference") (OtherBodyIndex :type Integer) (bFromSweep :type Boolean) (SweepResult :type "HitResult Structure (by ref)"))
  (if (`KismetSystemLibrary.DoesImplementInterface` OtherActor "/Game/Blueprints/BPI/BPI_FlashLight.BPI_FlashLight_C")
    (if (not (`KismetArrayLibrary.Array_Contains` (`ActorComponent.ComponentTags` OverlappedComponent) "ignor"))
      (message `/Game/Blueprints/BPI/BPI_FlashLight.HandleStartRechargeBattery` OtherActor))))

(event `self.Box.OnComponentEndOverlap`
  (params (OverlappedComponent :type "PrimitiveComponent Object Reference") (OtherActor :type "Actor Object Reference") (OtherComp :type "PrimitiveComponent Object Reference") (OtherBodyIndex :type Integer))
  (if (`KismetSystemLibrary.DoesImplementInterface` OtherActor "/Game/Blueprints/BPI/BPI_FlashLight.BPI_FlashLight_C")
    (if (not (`KismetArrayLibrary.Array_Contains` (`ActorComponent.ComponentTags` OverlappedComponent) "ignor"))
      (message `/Game/Blueprints/BPI/BPI_FlashLight.HandleEndRechargingBattery` OtherActor))))

(fn `UserConstructionScript`)