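; BP_egg is a VR cooking item that cracks when it hits something hard enough.
; On a BaseItem hit, it checks its speed against a threshold, ignores actors tagged VR_Player, and requires CanCrack, which is set once it leaves its spawn point.
; After a short delay, a one-shot guard lets it spawn two eggshells and a yolk at component transforms, then destroy itself.
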(event `self.ReceiveBeginPlay`
  (`parent.ReceiveBeginPlay`))

(event `self.ReceiveTick`
  (params (DeltaSeconds :type "Float (single-precision)"))
  (`parent.ReceiveTick` DeltaSeconds))

(event `self.BaseItem.OnComponentHit`
  (params (HitComponent :type "PrimitiveComponent Object Reference") (OtherActor :type "Actor Object Reference") (OtherComp :type "PrimitiveComponent Object Reference") (NormalImpulse :type "Vector Structure") (Hit :type "HitResult Structure (by ref)"))
  (bind _returnvalue (`PrimitiveComponent.GetPhysicsLinearVelocity` (`self.BaseItem`) "None"))
  (if (and (> (`KismetMathLibrary.VSize` _returnvalue) 50.0) (not (`self.ActorHasTag` OtherActor "VR_Player")) (`self.Can crack?`))
    (`KismetSystemLibrary.Delay` 0.1)
    (if (not (`self.Did crack?`))
      (set `self.Did crack?` true)
      (`|SpawnActorFromClass` "/Game/Blueprints/CookingItems/Snacks/BP_eggshell.BP_eggshell_C" (`SceneComponent.K2_GetComponentToWorld` (`self.1`)) "Undefined" "MultiplyWithRoot" null true null)
      (`|SpawnActorFromClass` "/Game/Blueprints/CookingItems/Snacks/BP_eggshell.BP_eggshell_C" (`SceneComponent.K2_GetComponentToWorld` (`self.2`)) "Undefined" "MultiplyWithRoot" null true null)
      (`|SpawnActorFromClass` "/Game/Blueprints/CookingItems/Snacks/BP_eggYolk.BP_eggYolk_C" (`SceneComponent.K2_GetComponentToWorld` (`self.yolk`)) "Undefined" "MultiplyWithRoot" null true null)
      (`self.K2_DestroyActor`))))

(event `/Game/Blueprints/BPI/BPI_BaseItem.LeftSpawnPoint`
  (set `self.Can crack?` true))

(fn `UserConstructionScript`
  (`parent.UserConstructionScript`))