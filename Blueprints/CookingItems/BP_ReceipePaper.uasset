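; BP_ReceipePaper is a recipe paper actor that displays an order card through a widget component.
; On BeginPlay it calls its parent, creates a W_Receipt widget, stores it, and assigns it to the Widget component.
; It then passes its OrderData to the receipt with SetOrderToCard, so the card is filled once at spawn with no Tick logic.
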(event `self.ReceiveBeginPlay`
  (`parent.ReceiveBeginPlay`)
  (bind _returnvalue (`|CreateWidget` "/Game/Blueprints/GamePlay/W_Receipt.W_Receipt_C"))
  (set `self.W_Receipt` _returnvalue)
  (`WidgetComponent.SetWidget` (`self.Widget`) (`self.W_Receipt`))
  (`/Game/Blueprints/GamePlay/W_Receipt.SetOrderToCard` (`self.W_Receipt`) (`self.OrderData`)))

(fn `UserConstructionScript`
  (`parent.UserConstructionScript`))