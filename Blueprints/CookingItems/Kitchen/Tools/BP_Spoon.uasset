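; BP_Spoon is a kitchen cooking tool that interacts with containers and displays a scoop of "Gup" while carrying an item.
; Outside flat mode, a sphere overlap with "container"-tagged components calls BPCTool's interaction; flat mode forwards grabbed-object interactions to the same component.
; Grab and remove events toggle the Gup's visibility, with a map from item data asset to scalar parameter setting its dynamic material's look.
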(event `self.ReceiveBeginPlay`
  (`parent.ReceiveBeginPlay`)
  (`/Game/Blueprints/BPC/BPC_Tool.Init` (`self.BPC_Tool`) self)
  (bind _returnvalue (`PrimitiveComponent.CreateDynamicMaterialInstance` (`self.Gup`) 0 "/Game/Materials/Textures/Scoop/Gup/M_SpoonGup.M_SpoonGup" "None"))
  (set `self.M_GupMaterialInstance` _returnvalue))

(event `self.Sphere_0.OnComponentBeginOverlap`
  (params (OverlappedComponent :type "PrimitiveComponent Object Reference") (OtherActor :type "Actor Object Reference") (OtherComp :type "PrimitiveComponent Object Reference") (OtherBodyIndex :type Integer) (bFromSweep :type Boolean) (SweepResult :type "HitResult Structure (by ref)"))
  (if (`/Game/Blueprints/BPFL/BPFL_GlobalFunctions.IsFlatmode`)
    _
    (elif (`KismetArrayLibrary.Array_Contains` (`ActorComponent.ComponentTags` OtherComp) "container")
      (`/Game/Blueprints/BPFL/BPFL_GlobalFunctions.Debug - Print string` (`KismetSystemLibrary.GetDisplayName` OtherActor) false)
      (`/Game/Blueprints/BPC/BPC_Tool.TryIneract` (`self.BPC_Tool`) OtherActor))))

(event `/Game/Blueprints/BPI/BPI_Interaction.FM_InterectToGrabedObject`
  (params (Actor :type "Actor Object Reference"))
  (if (not (== Actor "BP_Spoon"))
    (`/Game/Blueprints/BPC/BPC_Tool.TryIneract` (`self.BPC_Tool`) Actor)))

(event `/Game/Blueprints/BPI/BPI_Tool.GupHasBeenGrabed`
  (params (DA_Item :type "/Game/Blueprints/DataAssets/Items/DA_Item Object Reference"))
  (bind (_value _returnvalue) (`BlueprintMapLibrary.Map_Find` (`self.GupTypeMaterial`) DA_Item))
  (`|ExecutionSequence`
    (:`then_0`
      (if _returnvalue
        (`MaterialInstanceDynamic.SetScalarParameterValue` (`self.M_GupMaterialInstance`) "Value" (`KismetMathLibrary.Conv_IntToDouble` _value))))
    (:`then_1`
      (`SceneComponent.SetVisibility` (`self.Gup`) true false))))

(event `/Game/Blueprints/BPI/BPI_Tool.GupHasBeenRemoved`
  (`SceneComponent.SetVisibility` (`self.Gup`) false false))

(fn `FlatMode_Interaction`
  (returns (BaseItemMasterRef :type "/Game/Blueprints/CookingItems/A_BP_BaseItem_Master Object Reference") (InteractionType :type "/Game/Blueprints/Enums/E_InteractionTypes Enum") (Actor :type "Actor Object Reference"))
  (return self "NewEnumerator0" self))

(fn `GetGupMaterial`
  (returns (NewParam :type "MaterialInstanceDynamic Object Reference")))

(fn `UserConstructionScript`
  (`parent.UserConstructionScript`))