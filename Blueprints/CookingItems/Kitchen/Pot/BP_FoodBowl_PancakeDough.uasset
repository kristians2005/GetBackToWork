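; BP_FoodBowl_PancakeDough is a cooking food bowl of pancake dough that can turn into finished pancakes.
; ChangeToPankcakes converts it only once, returning true on success and false if it is already pancakes.
; The conversion event sets the flag, hides the bowl batter mesh, shows three pancake meshes, activates warm smoke and sets the container component's final food item to the pancake data asset.
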(event `ChangeMeshToPankcake`
  (set `self.IsPancakeNow?` true)
  (`SceneComponent.SetVisibility` (`self.BowlGup`) false false)
  (`SceneComponent.SetVisibility` (`self.Pancake1`) true false)
  (`SceneComponent.SetVisibility` (`self.Pancake2`) true false)
  (`SceneComponent.SetVisibility` (`self.Pancake3`) true false)
  (`ActorComponent.Activate` (`self.NS_WarmSmoke`) true)
  (set `/Game/Blueprints/BPC/BPC_Container_V2.FinalContainerFoodItem` "/Game/Blueprints/DataAssets/Items/Foods/DA_Pancake.DA_Pancake" (`self.BPC_Container_V2`)))

(fn `ChangeToPankcakes`
  (returns (Success :type Boolean))
  (if (`self.IsPancakeNow?`)
    (return false)
    (else
      (`self.ChangeMeshToPankcake`)
      (return true))))

(fn `UserConstructionScript`
  (`parent.UserConstructionScript`))