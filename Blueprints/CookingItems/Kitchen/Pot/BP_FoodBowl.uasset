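; BP_FoodBowl is a kitchen food bowl that hands out food and displays stacked pancakes.
; GetFoodDA takes an ingredient from BPCContainerV2 when allowed and returns its data asset.
; StackItems_1 responds to the "pancake" tag by incrementing a counter and revealing the pancake mesh at that index.
; Each revealed mesh gets a dynamic material whose Cooked_State parameter reflects raw, cooked or burnt.
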(event `self.ReceiveBeginPlay`
  (`parent.ReceiveBeginPlay`)
  (`KismetArrayLibrary.Array_Add` (`self.PancakeMesh`) (`self.Pancake1`))
  (`KismetArrayLibrary.Array_Add` (`self.PancakeMesh`) (`self.Pancake2`))
  (`KismetArrayLibrary.Array_Add` (`self.PancakeMesh`) (`self.Pancake3`)))

(event `StackItems_1`
  (params (tag :type Name) (CookedState :type "/Game/Blueprints/Enums/E_CookingState Enum" :default "NewEnumerator0"))
  (bind _output (`|GetArrayItem` (`self.PancakeMesh`) (`self.PancakeStackAmount`)))
  (if (== tag "pancake")
    (set `self.PancakeStackAmount` (+ (`self.PancakeStackAmount`) 1))
    (`/Engine/EditorBlueprintResources/StandardMacros.IsValid` _output
      (:`Is Valid`
        (`SceneComponent.SetVisibility` _output true false)
        (bind _returnvalue (`PrimitiveComponent.CreateDynamicMaterialInstance` _output 0 (`PrimitiveComponent.GetMaterial` _output 0) "None"))
        (`MaterialInstanceDynamic.SetScalarParameterValue` _returnvalue "Cooked_State" (select `/Game/Blueprints/Enums/E_CookingState` CookedState :`NewEnumerator1` 1.0 :`NewEnumerator2` 2.0))
        (`/Game/Blueprints/BPFL/BPFL_GlobalFunctions.Debug - Print string` "asdas")))))

(fn `GetFoodDA`
  (returns (Data :type "/Game/Blueprints/DataAssets/Items/DA_Item Object Reference") (success :type Boolean) (`AmountJustOne?` :type Boolean))
  (bind _bpc_container_v2 (`self.BPC_Container_V2`))
  (bind _success (`/Game/Blueprints/BPC/BPC_Container_V2.CanTakeFood?` _bpc_container_v2))
  (if _success
    (bind (_success_2 _da_item _amountjustone_) (`/Game/Blueprints/BPC/BPC_Container_V2.TakeIngredient` _bpc_container_v2))
    (return _da_item _success_2 _amountjustone_)
    (else
      (return null false false))))

(fn `UserConstructionScript`
  (`parent.UserConstructionScript`))