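; Base drink cup for the cooking system that fills with juices, shows the liquid level and spills when tilted.
; Pouring tracks amounts per juice, blends their colors into a dynamic liquid material and adds ingredient tags for recipe queries.
; Tick caps fill height by tilt, taken from the up-vector dot product, and clears juices once empty.
; A nearly full cup gets a lid that stops spilling; hot drinks emit smoke.
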(event `self.ReceiveBeginPlay`
  (`parent.ReceiveBeginPlay`)
  (`|ExecutionSequence`
    (:`then_0`
      (bind _returnvalue (`PrimitiveComponent.CreateDynamicMaterialInstance` (`self.BaseItem`) (`self.CupLiquidMateralIndex`) "/Game/Materials/Textures/M_Liquid.M_Liquid" "None"))
      (set `self.M_LiquidRef` _returnvalue)
      (`self.SetLuiqidHeight` (`self.FillHeight`)))
    (:`then_1`
      (if (not (`KismetArrayLibrary.Array_IsEmpty` (`self.Contents`)))
        (for _array_element (`self.Contents`)
          (`BlueprintGameplayTagLibrary.AppendGameplayTagContainers` (`self.CupTags`) (`/Game/Blueprints/DataAssets/Items/DA_Item.Ingredient-Tags` _array_element)))
        (`/Game/Blueprints/BPFL/BPFL_GlobalFunctions.Debug - Print string` (`BlueprintGameplayTagLibrary.GetDebugStringFromGameplayTagContainer` (`self.CupTags`)) false)))))

(event `self.ReceiveTick`
  (params (DeltaSeconds :type "Float (single-precision)"))
  (bind _fillheight (`self.FillHeight`))
  (`parent.ReceiveTick` DeltaSeconds)
  ;[0.15 0.06242 0.007204 0.5] Update Liquid state
  (`KismetSystemLibrary.Delay` DeltaSeconds)
  (if (`self.CanSpill?`)
    (if (> _fillheight 0.0)
      (if (> _fillheight (`self.LiquidSpillTilt`))
        (`self.SetLuiqidHeight` (`self.LiquidSpillTilt`))
        (if (and (`self.Is Hot`) (`ActorComponent.IsActive` (`self.HotDrinkSmokeParticles`)) (< (`self.FillHeight`) 1.0))
          (`KismetSystemLibrary.Delay` 2.0)
          (`ActorComponent.Deactivate` (`self.HotDrinkSmokeParticles`))))
      (elif (not (`BlueprintMapLibrary.Map_IsEmpty` (`self.JuiceContents`)))
        (`BlueprintMapLibrary.Map_Clear` (`self.JuiceContents`))
        (`KismetArrayLibrary.Array_Clear` (`self.AllJuiceColors`))))))

(event `/Game/Blueprints/BPI/BPI_Interaction.SetLiquidHeight`
  (params (`LiquidHeight (0 - 10)` :type "Float (double-precision)"))
  (`self.SetLuiqidHeight` `LiquidHeight (0 - 10)`))

(event `/Game/Blueprints/BPI/BPI_Interaction.FillCupWithLiquid`
  (params (FillAmount :type "Float (double-precision)") (JuiceType :type "/Game/Blueprints/DataAssets/Items/DA_Item Object Reference") (`IsDrinkHot?` :type Boolean))
  ; Fill cup with fluid
  (set `self.Is Hot` `IsDrinkHot?`)
  (if (> (`self.FillHeight`) 8.8)
    (`|ExecutionSequence`
      (:`then_0`
        (`/Engine/EditorBlueprintResources/StandardMacros.DoOnce` false
          (:`Completed`
            (set `self.CanSpill?` false)
            (`SceneComponent.SetVisibility` (`self.lid`) true false)
            ;[0.06281 0.15 0.0719 0.5] increase liquid height
            (`GameplayStatics.SpawnSoundAtLocation` "/Game/Sound/SFX2/fly_generic_plastic_grab_05.fly_generic_plastic_grab_05" (`SceneComponent.K2_GetComponentLocation` (`self.BaseItem`)) (struct) 1.0 1.0 0.0 null null))))
      (:`then_1`
        _)))
  (if (< (`self.FillHeight`) 8.9)
    (bind _output_get (set `self.FillHeight` (+ (`self.FillHeight`) FillAmount)))
    (`self.SetLuiqidHeight` _output_get))
  ;[0.06301 0.15 0.07227 0.5] Add Juice to FluidContent
  (if (`BlueprintMapLibrary.Map_Contains` (`self.JuiceContents`) JuiceType)
    (`BlueprintMapLibrary.Map_Add` (`self.JuiceContents`) JuiceType (+ (`BlueprintMapLibrary.Map_Find` (`self.JuiceContents`) JuiceType) FillAmount))
    (if (> (`BlueprintMapLibrary.Map_Find` (`self.JuiceContents`) JuiceType) 2.0)
      (`self.AddIngredient` JuiceType))
    (else
      (`BlueprintMapLibrary.Map_Add` (`self.JuiceContents`) JuiceType FillAmount)
      (`KismetArrayLibrary.Array_Add` (`self.AllJuiceColors`) (`/Game/Blueprints/DataAssets/Items/DA_Item.Color` JuiceType))
      (if (< (`BlueprintMapLibrary.Map_Length` (`self.JuiceContents`)) 1)
        (`self.AddIngredient` JuiceType))))
  (if true
    (`self.BlendMixedLiquidColors`)
    (if (and (`self.Is Hot`) (not (`ActorComponent.IsActive` (`self.HotDrinkSmokeParticles`))) (> (`self.FillHeight`) 4.0))
      (`ActorComponent.Activate` (`self.HotDrinkSmokeParticles`) true))))

(event `RecipeManager`)

(fn `AddIngredient`
  (params (Ingredient :type "/Game/Blueprints/DataAssets/Items/DA_Item Object Reference"))
  (`KismetArrayLibrary.Array_Add` (`self.Contents`) Ingredient)
  (`BlueprintGameplayTagLibrary.AppendGameplayTagContainers` (`self.CupTags`) (`/Game/Blueprints/DataAssets/Items/DA_Item.Ingredient-Tags` Ingredient))
  (return))

(fn `BlendMixedLiquidColors`
  (locals (LocalMixedColor :type "Array of LinearColor Structure"))
  (bind (_liquidcolor_r _liquidcolor_g _liquidcolor_b) (break `LinearColor` (`self.LiquidColor`)))
  (bind _values (`BlueprintMapLibrary.Map_Values` (`self.JuiceContents`)))
  (for (_array_element _array_index) _values
    (bind (_output_r _output_g _output_b) (break `LinearColor` (`|GetArrayItem` (`self.AllJuiceColors`) _array_index)))
    (bind _returnvalue (`KismetMathLibrary.MapRangeClamped` _array_element 0.0 (`self.FillHeight`) 0.0 1.0))
    (`KismetArrayLibrary.Array_Add` (`local.LocalMixedColor`) (make `LinearColor` (* _output_r _returnvalue) (* _output_g _returnvalue) (* _output_b _returnvalue) 1.0)))
  (for (_array_element_2 _array_index_2) (`local.LocalMixedColor`)
    (if (== _array_index_2 0)
      (set `self.LiquidColor` _array_element_2)
      (else
        (bind (_r _g _b) (`KismetMathLibrary.BreakColor` _array_element_2))
        (set `self.LiquidColor` (make `LinearColor` (+ _r _liquidcolor_r) (+ _g _liquidcolor_g) (+ _b _liquidcolor_b) 1.0)))))
  (`MaterialInstanceDynamic.SetVectorParameterValue` (`self.M_LiquidRef`) "LiquidColor" (`self.LiquidColor`)))

(fn `GetAll_DA_items`
  (returns (NewParam :type "Array of /Game/Blueprints/DataAssets/Items/DA_Item Object Reference"))
  (locals (L_DaItem :type "Array of /Game/Blueprints/DataAssets/Items/DA_Item Object Reference"))
  (`KismetArrayLibrary.Array_Add` (`local.L_DaItem`) (`self.Item`))
  (for _array_element (`/Game/Blueprints/BPC/BPC_Container_V2.Ingredients` (`self.BPC_Container_V2`))
    (`KismetArrayLibrary.Array_Add` (`local.L_DaItem`) _array_element))
  (bind _keys (`BlueprintMapLibrary.Map_Keys` (`self.JuiceContents`)))
  (for _array_element_2 _keys
    (`KismetArrayLibrary.Array_Add` (`local.L_DaItem`) _array_element_2))
  (return (`local.L_DaItem`)))

(fn `GetDAItem`
  (returns (GetDAIten :type "/Game/Blueprints/DataAssets/Items/DA_Item Object Reference"))
  (if (> (`self.FillHeight`) 7.0)
    (bind _keys (`BlueprintMapLibrary.Map_Keys` (`self.JuiceContents`)))
    (return (`|GetArrayItem` _keys))
    (else
      (return "/Game/Blueprints/DataAssets/Items/Foods/DA_WRONGITEM.DA_WRONGITEM"))))

(fn `Getfood`
  (returns (NewParam :type "Array of /Game/Blueprints/DataAssets/Items/DA_Item Object Reference"))
  (return))

(fn `HandleReciveFood`
  (returns (FoodOrder :type "Array of Actor Object Reference"))
  (return))

(fn `LiquidSpillTilt`
  (returns (LiquidHeight :type "Float (double-precision)"))
  (return (`KismetMathLibrary.MapRangeClamped` (- 103.0 (`KismetMathLibrary.DegAcos` (`KismetMathLibrary.Dot_VectorVector` (`KismetMathLibrary.GetUpVector` (`SceneComponent.K2_GetComponentRotation` (`self.BaseItem`))) (0.0 0.0 1.0)))) 0.0 95.0 0.0 10.0)))

(fn `Recive item recipe Tags`
  (returns (Tags :type "GameplayTagContainer Structure"))
  (return (`self.CupTags`)))

(fn `SetLuiqidHeight`
  (params (FillHeight :type "Float (single-precision)"))
  (bind _output_get (set `self.FillHeight` FillHeight))
  (`MeshComponent.SetScalarParameterValueOnMaterials` (`self.BaseItem`) "Fill height" _output_get))

(fn `UserConstructionScript`
  (`parent.UserConstructionScript`)
  (bind _returnvalue (`PrimitiveComponent.CreateDynamicMaterialInstance` (`self.BaseItem`) (`self.CupLiquidMateralIndex`) "/Game/Materials/Textures/M_Liquid.M_Liquid" "None"))
  (`MaterialInstanceDynamic.SetVectorParameterValue` _returnvalue "LiquidColor" (`self.LiquidColor`))
  (`MeshComponent.SetScalarParameterValueOnMaterials` (`self.BaseItem`) "Fill height" (`self.FillHeight`)))