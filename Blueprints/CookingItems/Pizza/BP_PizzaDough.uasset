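; Pizza dough cooking item that is flattened in stages by hits from other base items, then becomes a cookable base for ingredients.
; Debounced hits, enabled by placement or flat mode, step through mesh states until the final one unlocks cooking.
; Outside flat mode, overlapping non-spoon items enter the container component and are destroyed, releasing them from VR hands.
; Its reported item is the container's final food or a wrong-item fallback, depending on cooked state.
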(event `self.ReceiveBeginPlay`
  (`parent.ReceiveBeginPlay`)
  (`self.ChangePizzaDoughState` (`|GetArrayItem` (`self.AllPizzaDoughStates`) (`self.PizzaDoughStateIndex`)))
  (set `self.CanAddNewIngredients` false)
  (if (`/Game/Blueprints/BPFL/BPFL_GlobalFunctions.IsFlatmode`)
    (set `self.CanBreak` true)))

(event `self.BaseItem.OnComponentHit`
  (params (HitComponent :type "PrimitiveComponent Object Reference") (OtherActor :type "Actor Object Reference") (OtherComp :type "PrimitiveComponent Object Reference") (NormalImpulse :type "Vector Structure") (Hit :type "HitResult Structure (by ref)"))
  (if (`KismetMathLibrary.ClassIsChildOf` (`GameplayStatics.GetObjectClass` OtherActor) "/Game/Blueprints/CookingItems/A_BP_BaseItem_Master.A_BP_BaseItem_Master_C")
    (if (`self.CanBreak`)
      (`/Engine/EditorBlueprintResources/StandardMacros.DoOnce` false :!label _label
        (:`Completed`
          (`|ExecutionSequence`
            (:`then_0`
              (set `self.PizzaDoughStateIndex` (+ (`self.PizzaDoughStateIndex`) 1))
              (if (>= (+ (`self.PizzaDoughStateIndex`) 0) (`KismetArrayLibrary.Array_Length` (`self.AllPizzaDoughStates`)))
                (if (not (`self.CanCook?`))
                  (`self.ChangePizzaDoughState` (`self.Item`))
                  (set `self.CanAddNewIngredients` true)
                  (set `self.CanBreak` false)
                  (set `self.CanCook?` true))
                (else
                  (`self.ChangePizzaDoughState` (`|GetArrayItem` (`self.AllPizzaDoughStates`) (`self.PizzaDoughStateIndex`))))))
            (:`then_1`
              (`KismetSystemLibrary.Delay` 0.4)
              (goto _label :!via `Reset`))))))))

(event `/Game/Blueprints/BPI/BPI_BaseItem.ItemTakenAway`
  (set `self.CanBreak` false))

(event `/Game/Blueprints/BPI/BPI_BaseItem.ItemPlacedDown`
  (set `self.CanBreak` true))

(event `self.Box.OnComponentBeginOverlap`
  (params (OverlappedComponent :type "PrimitiveComponent Object Reference") (OtherActor :type "Actor Object Reference") (OtherComp :type "PrimitiveComponent Object Reference") (OtherBodyIndex :type Integer) (bFromSweep :type Boolean) (SweepResult :type "HitResult Structure (by ref)"))
  (if (`KismetMathLibrary.ClassIsChildOf` (`GameplayStatics.GetObjectClass` OtherActor) "/Game/Blueprints/CookingItems/Kitchen/Tools/BP_Spoon.BP_Spoon_C")
    _
    (elif (`/Game/Blueprints/BPFL/BPFL_GlobalFunctions.IsFlatmode`)
      _
      (elif (`self.CanAddNewIngredients`)
        (bind _ref (message `/Game/Blueprints/BPI/BPI_BaseItem.GetBaseItemSelfRef` OtherActor))
        (`/Engine/EditorBlueprintResources/StandardMacros.IsValid` _ref
          (:`Is Valid`
            (bind _item (`/Game/Blueprints/CookingItems/A_BP_BaseItem_Master.Item` _ref))
            (bind _success_ (`/Game/Blueprints/BPC/BPC_Container_V2.AddNewIngredient` (`self.BPC_Container_V2`) _item (`/Game/Blueprints/DataAssets/Items/DA_Item.AddAmountJustOne` _item) "NewEnumerator0" true))
            (if _success_
              (if (`/Game/Game_BP/VRTemplate/Blueprints/GrabComponent.bIsHeld` (`/Game/Blueprints/CookingItems/A_BP_BaseItem_Master.GrabComponent` _ref))
                (message `/Game/Blueprints/BPI/BPI_Interaction.VR_ReleaseFromHand` (`GameplayStatics.GetPlayerCharacter` 0) (`/Game/Game_BP/VRTemplate/Blueprints/GrabComponent.GetHeldByHand` (`/Game/Blueprints/CookingItems/A_BP_BaseItem_Master.GrabComponent` _ref)))
                (`self.K2_DestroyActor` _ref)
                (else
                  (`self.K2_DestroyActor` _ref))))))))))

(fn `CanBeCooked?`
  (returns (`Success?` :type Boolean))
  (return (`self.CanCook?`)))

(fn `ChangePizzaDoughState`
  (params (Item :type "/Game/Blueprints/DataAssets/Items/DA_Item Object Reference"))
  (bind _mesh (`/Game/Blueprints/DataAssets/Items/DA_Item.Mesh` Item))
  (`/Engine/EditorBlueprintResources/StandardMacros.IsValid` Item
    (:`Is Valid`
      (`StaticMeshComponent.SetStaticMesh` (`self.BaseItem`) _mesh)
      (`PrimitiveComponent.SetMaterial` (`self.BaseItem`) 0 (`StaticMesh.GetMaterial` _mesh 0)))))

(fn `GetDAItem`
  (returns (GetDAIten :type "/Game/Blueprints/DataAssets/Items/DA_Item Object Reference"))
  (if (`|EnumEquality` (`/Game/Blueprints/BPC/BPC_Cooking_V2.CookedState` (`self.BPC_Cooking_V2`)) "NewEnumerator1")
    (return (`/Game/Blueprints/BPC/BPC_Container_V2.FinalContainerFoodItem` (`self.BPC_Container_V2`)))
    (else
      (return "/Game/Blueprints/DataAssets/Items/Foods/DA_WRONGITEM.DA_WRONGITEM"))))

(fn `UserConstructionScript`
  (`parent.UserConstructionScript`))