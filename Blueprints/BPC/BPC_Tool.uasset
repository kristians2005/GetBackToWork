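; BPC_Tool is a component that lets its owning tool pick up a food item and pass it to ovens, providers and containers.
; TryIneract checks the target's interfaces: oven receivers get the held item, while dual provider-receivers take or give depending on whether one is held.
; Transfers go through interface messages, exclude DA_Spoon when taking or giving, and notify the owner when the "Gup" is grabbed or removed.
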(event `Init`
  (params (AcrorRef :type "/Game/Blueprints/CookingItems/A_BP_BaseItem_Master Object Reference"))
  (set `self.Self Acror Ref` AcrorRef))

(event `TryIneract`
  (params (OtherActor :type "Actor Object Reference"))
  (bind _other_actor (`self.Other Actor`))
  (`/Engine/EditorBlueprintResources/StandardMacros.IsValid` OtherActor
    (:`Is Valid`
      (set `self.Other Actor` OtherActor)
      (if (`KismetSystemLibrary.DoesImplementInterface` (`self.Other Actor`) "/Game/Blueprints/BPI/BPI_OvenFoodReciver.BPI_OvenFoodReciver_C")
        (`self.PLaceFoodOnOven`)
        (elif (and (`KismetSystemLibrary.DoesImplementInterface` _other_actor "/Game/Blueprints/BPI/BPI_FoodProvider.BPI_FoodProvider_C") (`KismetSystemLibrary.DoesImplementInterface` _other_actor "/Game/Blueprints/BPI/BPI_FoodReciver.BPI_FoodReciver_C"))
          (if (`KismetSystemLibrary.IsValid` (`self.DA_Item`))
            (`self.GiveFoodToContainer`)
            (else
              (`self.TakeFood`)))
          (elif (`KismetSystemLibrary.DoesImplementInterface` (`self.Other Actor`) "/Game/Blueprints/BPI/BPI_FoodProvider.BPI_FoodProvider_C")
            (`self.TakeFood`)
            (else
              (`self.GiveFoodToContainer`))))))))

(event `PLaceFoodOnOven`
  (if (not (not (`KismetSystemLibrary.IsValid` (`self.DA_Item`))))
    (bind _success (message `/Game/Blueprints/BPI/BPI_OvenFoodReciver.TryPlaceFoodOnOven` (`self.Other Actor`) (`self.DA_Item`)))
    (if _success
      (set `self.DA_Item` null)
      (message `/Game/Blueprints/BPI/BPI_Tool.GupHasBeenRemoved` (`self.Self Acror Ref`)))))

(event `TakeFood`
  (bind (_data _success _amountjustone_) (message `/Game/Blueprints/BPI/BPI_FoodProvider.GetFoodDA` (`self.Other Actor`)))
  (if _success
    (`/Engine/EditorBlueprintResources/StandardMacros.IsValid` _data
      (:`Is Valid`
        (set `self.AmountJustOne?` _amountjustone_)
        (if (not (== _data "/Game/Blueprints/DataAssets/Items/Containers/DA_Spoon.DA_Spoon"))
          (bind _output_get (set `self.DA_Item` _data))
          (message `/Game/Blueprints/BPI/BPI_Tool.GupHasBeenGrabed` (`self.Self Acror Ref`) _output_get))))))

(event `GiveFoodToContainer`
  (`/Engine/EditorBlueprintResources/StandardMacros.IsValid` (`self.DA_Item`)
    (:`Is Valid`
      (if (not (== (`self.DA_Item`) "/Game/Blueprints/DataAssets/Items/Containers/DA_Spoon.DA_Spoon"))
        (bind _success_ (message `/Game/Blueprints/BPI/BPI_FoodReciver.GiveFoodDataToTarget` (`self.Other Actor`) (`self.DA_Item`) (`self.AmountJustOne?`)))
        (if _success_
          (set `self.DA_Item` null)
          (message `/Game/Blueprints/BPI/BPI_Tool.GupHasBeenRemoved` (`self.Self Acror Ref`)))))))

(fn `GetFoodDA`
  (returns (Data :type "/Game/Blueprints/DataAssets/Items/DA_Item Object Reference") (success :type Boolean) (`AmountJustOne?` :type Boolean))
  (return null false false))

(fn `GetGupMaterial`
  (returns (NewParam :type "MaterialInstanceDynamic Object Reference"))
  (return null))

(fn `GiveFoodDataToTarget`
  (params (Data :type "/Game/Blueprints/DataAssets/Items/DA_Item Object Reference") (AmountJustOne :type Boolean)))

(fn `TryPlaceFoodOnOven`
  (params (DA_Item :type "/Game/Blueprints/DataAssets/Items/DA_Item Object Reference"))
  (returns (Success :type Boolean))
  (return false))