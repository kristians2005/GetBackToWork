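; Container component (BPC) that holds food ingredients for its owning actor and resolves which final food item they form.
; Init caches the owner's container item and ingredient meshes through interface messages, then adds any preset ingredients.
; Adding validates mesh tag, single-item amount and accepted cooked state, then shows the mesh and matches AllItem recipes by container and order-independent ingredients.
; TakeIngredient decrements the count, hiding the mesh when the last is taken.
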(event `Init`
  (params (Actor :type "Actor Object Reference"))
  (set `self.Self Ref` Actor)
  (bind _containeritem (message `/Game/Blueprints/BPI/BPI_Container_V2.GetContainerItem` (`self.Self Ref`)))
  (set `self.ContainerItem` _containeritem)
  (bind _meshesrefs (message `/Game/Blueprints/BPI/BPI_Container_V2.GetAllIngredientMeshRef` (`self.Self Ref`)))
  (set `self.Meshes Refs` _meshesrefs)
  (message `/Game/Blueprints/BPI/BPI_Container_V2.ToggleAllIngredientMeshVisibility` (`self.Self Ref`) (`self.Debug_InitVisible?`))
  (if (`KismetArrayLibrary.Array_IsNotEmpty` (`self.InitIngredients`))
    (`self.InitAddIngredients`)))

(fn `AddNewIngredient`
  (params (DA_Item :type "/Game/Blueprints/DataAssets/Items/DA_Item Object Reference") (`GiveAomuntJustone?` :type Boolean) (CookedState :type "/Game/Blueprints/Enums/E_CookingState Enum" :default "NewEnumerator0") (`PlaySound?` :type Boolean :default true))
  (returns (`success?` :type Boolean))
  (locals (L_DA_Item :type "/Game/Blueprints/DataAssets/Items/DA_Item Object Reference") (L_AmountJustOne :type Boolean) (L_CookedState :type "/Game/Blueprints/Enums/E_CookingState Enum" :default "NewEnumerator0") (L_PlaySound :type Boolean :default true))
  (bind _ingredients (`self.Ingredients`))
  (set `local.L_PlaySound` `PlaySound?`)
  (set `local.L_CookedState` CookedState)
  (set `local.L_AmountJustOne` `GiveAomuntJustone?`)
  (if (not (== DA_Item "/Game/Blueprints/DataAssets/Items/Containers/DA_Spoon.DA_Spoon"))
    (set `local.L_DA_Item` DA_Item)
    (bind _success_ (`self.CompareMeshTagTo-DA_Item` (`self.Meshes Refs`) (`/Game/Blueprints/DataAssets/Items/DA_Item.MeshFoodTag` (`local.L_DA_Item`))))
    (if _success_
      (if (`self.IsAmountSet?`)
        (if (<= (`self.Amount`) 0)
          (`KismetArrayLibrary.Array_Clear` (`self.Ingredients`))
          (set `self.IsAmountSet?` false)))
      (if (`/Game/Blueprints/DataAssets/Items/DA_Item.IsThisASingleItem` (`local.L_DA_Item`))
        ; Im fucing gonna start tweekin
        (if (or (== (`local.L_DA_Item`) (`|GetArrayItem` _ingredients)) (<= (`KismetArrayLibrary.Array_Length` _ingredients) 1))
          (if (!= (`/Game/Blueprints/DataAssets/Items/DA_Item.ItemAmount` (`local.L_DA_Item`)) 0)
            (set `self.IsAmountSet?` true)
            ; Good luck understanding whats going on here future me :(
            (if (`local.L_AmountJustOne`)
              (if (> (+ (`self.Amount`) 1) (`/Game/Blueprints/DataAssets/Items/DA_Item.ItemAmount` (`local.L_DA_Item`)))
                (return false)
                (else
                  (set `self.Amount` (+ (`self.Amount`) 1))))
              (else
                (set `self.Amount` (`/Game/Blueprints/DataAssets/Items/DA_Item.ItemAmount` (`local.L_DA_Item`))))))
          (else
            (return false))))
      (if (`self.CanOnlyHaveOneIngredient`)
        (return false)
        (else
          (set `self.CanOnlyHaveOneIngredient` (`/Game/Blueprints/DataAssets/Items/DA_Item.IsThisASingleItem` (`local.L_DA_Item`)))
          (bind _cookedstate (message `/Game/Blueprints/BPI/BPI_Container_V2.GetFoodCookedState` (`self.Self Ref`)))
          (bind _values (`BlueprintMapLibrary.Map_Values` (`self.WhatCookedStateItemsDoesItAccept?`)))
          (if (select `/Game/Blueprints/Enums/E_CookingState` _cookedstate :`NewEnumerator0` (`|GetArrayItem` _values) :`NewEnumerator1` (`|GetArrayItem` _values 1) :`NewEnumerator2` (`|GetArrayItem` _values 2))
            (if (not (`KismetArrayLibrary.Array_Contains` (`self.Ingredients`) (`local.L_DA_Item`)))
              (bind _success__2 (`self.CompareMeshTagTo-DA_Item` (`self.Meshes Refs`) (`/Game/Blueprints/DataAssets/Items/DA_Item.MeshFoodTag` (`local.L_DA_Item`))))
              (if _success__2
                (`KismetArrayLibrary.Array_Add` (`self.Ingredients`) (`local.L_DA_Item`))
                (message `/Game/Blueprints/BPI/BPI_Container_V2.ToggleIngredientVisibilityByTag` (`self.Self Ref`) (`/Game/Blueprints/DataAssets/Items/DA_Item.MeshFoodTag` (`local.L_DA_Item`)) true (`/Game/Blueprints/DataAssets/Items/DA_Item.Stackable?` (`local.L_DA_Item`)) (`local.L_CookedState`))
                (`self.MatchAllItem`)
                (`self.PlaySoundSFX` (`self.Self Ref`) (`local.L_PlaySound`))
                (return true)
                (else
                  (return false)))
              (elif (`/Game/Blueprints/DataAssets/Items/DA_Item.IsThisASingleItem` (`local.L_DA_Item`))
                (if (`/Game/Blueprints/DataAssets/Items/DA_Item.Stackable?` (`local.L_DA_Item`))
                  (message `/Game/Blueprints/BPI/BPI_Container_V2.ToggleIngredientVisibilityByTag` (`self.Self Ref`) (`/Game/Blueprints/DataAssets/Items/DA_Item.MeshFoodTag` (`local.L_DA_Item`)) true (`/Game/Blueprints/DataAssets/Items/DA_Item.Stackable?` (`local.L_DA_Item`)) (`local.L_CookedState`))
                  (`self.MatchAllItem`)
                  (`self.PlaySoundSFX` (`self.Self Ref`) (`local.L_PlaySound`))
                  (return true)
                  (else
                    (`self.PlaySoundSFX` (`self.Self Ref`) (`local.L_PlaySound`))
                    (return true)))
                (else
                  (return false))))
            (else
              (return false)))))
      (else
        (return false)))))

(fn `CanTakeFood?`
  (returns (success :type Boolean))
  (if (`self.IsAmountSet?`)
    (if (<= (`self.Amount`) 0)
      (return false)
      (else
        (return true)))
    (else
      (return false))))

(fn `CompareMeshTagTo-DA_Item`
  (params (Array :type "Array of SceneComponent Object Reference") (Tag :type Name))
  (returns (`success?` :type Boolean) (Component :type "SceneComponent Object Reference"))
  (for _array_element Array
    (if (`KismetArrayLibrary.Array_Contains` (`ActorComponent.ComponentTags` _array_element) Tag)
      (return true _array_element)))
  (return false null))

(fn `GetAllIngredientMeshRef`
  (returns (MeshesRefs :type "Array of SceneComponent Object Reference"))
  (return))

(fn `GetContainerItem`
  (returns (Containeritem :type "/Game/Blueprints/DataAssets/Items/DA_Item Object Reference"))
  (return null))

(fn `GetFoodCookedState`
  (returns (CookedState :type "/Game/Blueprints/Enums/E_CookingState Enum"))
  (return "NewEnumerator0"))

(fn `GetIngredient`)

(fn `InitAddIngredients`
  (bind _initingredients (`self.InitIngredients`))
  (for _array_element _initingredients
    (if (`/Game/Blueprints/DataAssets/Items/DA_Item.IsThisASingleItem` _array_element)
      (`self.AddNewIngredient` _array_element false "NewEnumerator0" false)
      (return)))
  (for _array_element_2 _initingredients
    (`self.AddNewIngredient` _array_element_2 false "NewEnumerator0" false)))

(fn `MatchAllItem`
  (locals (Index :type Integer))
  (for _array_element (`self.AllItem`)
    (if (== (`self.ContainerItem`) (`/Game/Blueprints/DataAssets/Container/DA_Container.ContainerItem` _array_element))
      (if (== (`KismetArrayLibrary.Array_Length` (`.Ingredients_5_C938C1934B298E100DA4669AF9B1BBFF` (break `/Game/Blueprints/DataAssets/Container/ST_Container` (`/Game/Blueprints/DataAssets/Container/DA_Container.Ingredients` _array_element)))) (`KismetArrayLibrary.Array_Length` (`self.Ingredients`)))
        (set `local.Index` 0)
        (for _array_element_2 (`self.Ingredients`)
          (bind _ingredients (break `/Game/Blueprints/DataAssets/Container/ST_Container` (`/Game/Blueprints/DataAssets/Container/DA_Container.Ingredients` _array_element)))
          (if (`KismetArrayLibrary.Array_Contains` _ingredients _array_element_2)
            (set `local.Index` (+ (`local.Index`) 1))))
        (if (== (`KismetArrayLibrary.Array_Length` _ingredients) (`local.Index`))
          (bind _finalitem (`/Game/Blueprints/DataAssets/Container/DA_Container.FinalItem` _array_element))
          (`/Game/Blueprints/BPFL/BPFL_GlobalFunctions.Debug - Print string` (`KismetTextLibrary.Conv_TextToString` (`|FormatText` "{f}__{s}__{d}" (`self.Self Ref`) _finalitem (`local.Index`))) false (struct :`R` 1.0 :`G` 0.319719 :`B` 0.607567 :`A` 1.0))
          (set `self.FinalContainerFoodItem` _finalitem)
          (`/Game/Blueprints/BPFL/BPFL_GlobalFunctions.Debug - Print string` (`KismetSystemLibrary.GetDisplayName` _finalitem) false)
          (return))))))

(fn `PlaySoundSFX`
  (params (self2 :type "Object Object Reference") (yes :type Boolean))
  (if yes
    (message `/Game/Blueprints/BPI/BPI_Container_V2.PlaySound` self2))
  (return))

(fn `TakeIngredient`
  (returns (success :type Boolean) (DA_Item :type "/Game/Blueprints/DataAssets/Items/DA_Item Object Reference") (`AmountJustOne?` :type Boolean))
  (bind _amount (`self.Amount`))
  (`/Game/Blueprints/BPFL/BPFL_GlobalFunctions.Debug - Print string` (`KismetTextLibrary.Conv_TextToString` (`|FormatText` "{1}: {2}" (`|GetArrayItem` (`self.Ingredients`)) _amount)) true (struct :`R` 1.0 :`G` 0.52802 :`B` 0.701364 :`A` 1.0))
  (if (<= _amount 0)
    (return false null true)
    (else
      (if (== (`self.Amount`) 1)
        (message `/Game/Blueprints/BPI/BPI_Container_V2.ToggleIngredientVisibilityByTag` (`self.Self Ref`) (`/Game/Blueprints/DataAssets/Items/DA_Item.MeshFoodTag` (`|GetArrayItem` (`self.Ingredients`))) false false "NewEnumerator0"))
      (set `self.Amount` (- (`self.Amount`) 1))
      (return true (`|GetArrayItem` (`self.Ingredients`)) true))))