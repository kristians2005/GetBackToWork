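; Oven component, judging by the BPC prefix, that handles placing data-asset items onto its owning oven actor.
; Init caches that actor, and PlaceItemToOven looks the item up in the PhysicalPlacedItemOnOven map.
; A match is passed to the actor through the SpawnItemOnOven interface message, leaving the spawn itself to the actor.
; TryPlaceFoodOnOven is a stub that always returns false.
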(event `Init`
  (params (Actor :type "Actor Object Reference"))
  (set `self.SelfRef` Actor))

(fn `PlaceItemToOven`
  (params (DA_Item :type "/Game/Blueprints/DataAssets/Items/DA_Item Object Reference"))
  (returns (`Success?` :type Boolean))
  (locals (L_DA_Item :type "/Game/Blueprints/DataAssets/Items/DA_Item Object Reference"))
  (bind (_value _returnvalue) (`BlueprintMapLibrary.Map_Find` (`self.PhysicalPlacedItemOnOven`) (`local.L_DA_Item`)))
  (`/Engine/EditorBlueprintResources/StandardMacros.IsValid` DA_Item
    (:`Is Valid`
      (set `local.L_DA_Item` DA_Item)
      (if (not (not _returnvalue))
        (message `/Game/Blueprints/BPI/BPI_OvenFoodReciver.SpawnItemOnOven` (`self.SelfRef`) _value)
        (return true)))
    (:`Is Not Valid`
      (return false))))

(fn `TryPlaceFoodOnOven`
  (params (DA_Item :type "/Game/Blueprints/DataAssets/Items/DA_Item Object Reference"))
  (returns (Success :type Boolean))
  (return false))