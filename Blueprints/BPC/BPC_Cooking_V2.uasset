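; Cooking component that tracks a food actor's heat and switches it between raw, cooked and burnt.
; Looping timers raise Heat during heating and lower it afterwards, with the cooked state gated by oven type compatibility.
; State changes set Cooked_State on dynamic materials of the base and ingredient meshes, with burnt as final.
; The owning actor supplies meshes, oven compatibility and smoke control through messages.
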(event `Init`
  (params (Actor :type "Actor Object Reference"))
  (set `self.ActorRef` Actor))

(event `StartHetingFood`
  (params (OvenType :type "/Game/Blueprints/Enums/E_WhatOvenCanCook Enum" :default "NewEnumerator0"))
  (set `self.Oven Type` OvenType)
  (`KismetSystemLibrary.K2_ClearAndInvalidateTimerHandle` (`self.DecreaseTemperatureTimeFunction`))
  (bind _returnvalue (`KismetSystemLibrary.K2_SetTimer` null "IncreaseTemperature" 0.1 true))
  (set `self.IncreaseTemperature_TimerFunction` _returnvalue))

(event `EndHeatingFood`
  (`KismetSystemLibrary.K2_ClearAndInvalidateTimerHandle` (`self.IncreaseTemperature_TimerFunction`))
  (bind _returnvalue (`KismetSystemLibrary.K2_SetTimer` null "DecreaseTemperature" 0.5 true))
  (set `self.DecreaseTemperatureTimeFunction` _returnvalue))

(event `IncreaseTemperature`
  (if (< (`self.Heat`) (`self.BurntFoodState`))
    (if (< (`self.Heat`) (`self.CookedFoodState`))
      (set `self.Heat` (+ (`self.Heat`) (`self.CookingOvenHeat`)) :!label _label)
      (else
        (bind _success_ (message `/Game/Blueprints/BPI/BPI_FoodCooking.ActivateSmoke` (`self.ActorRef`)))
        (if _success_
          (goto _label)
          (else
            (bind _whatoventype_ (message `/Game/Blueprints/BPI/BPI_FoodCooking.GetWhatOvenCanCook` (`self.ActorRef`)))
            (if (select `/Game/Blueprints/Enums/E_WhatOvenCanCook` _whatoventype_ :`NewEnumerator0` true)
              (`self.HandleMaterialChange` "NewEnumerator1" :!label _label_2)
              (elif (== (`|GetEnumeratorName` _whatoventype_) (`|GetEnumeratorName` (`self.Oven Type`)))
                (goto _label_2)
                (else
                  (set `self.Heat` 100.0))))))))
    (else
      (`self.HandleMaterialChange` "NewEnumerator2"))))

(event `DecreaseTemperature`
  (if (< (`self.Heat`) 20.0)
    (`/Engine/EditorBlueprintResources/StandardMacros.DoOnce` false :!label _label_3
      (:`Completed`
        (message `/Game/Blueprints/BPI/BPI_FoodCooking.DisableSmoke` (`self.ActorRef`))))
    (else
      (set `self.Heat` (- (`self.Heat`) 1.0))
      (goto _label_3 :!via `Reset`))))

(event `HandleMaterialChange`
  (params (NewParam :type "/Game/Blueprints/Enums/E_CookingState Enum" :default "NewEnumerator0"))
  (bind _cookedstate (`self.CookedState`))
  (bind _returnvalue (select `/Game/Blueprints/Enums/E_CookingState` (`self.CookedState`) :`NewEnumerator1` 1.0 :`NewEnumerator2` 2.0))
  (if (not (== (`|GetEnumeratorName` (`self.CookedState`)) (`|GetEnumeratorName` (select `/Game/Blueprints/Enums/E_CookingState` (`self.CookedState`) :`NewEnumerator0` "NewEnumerator2" :`NewEnumerator1` "NewEnumerator2" :`NewEnumerator2` "NewEnumerator2" :!type "/Game/Blueprints/Enums/E_CookingState Enum"))))
    (if (not (== (`|GetEnumeratorName` NewParam) (`|GetEnumeratorName` (`self.CookedState`))))
      (set `self.CookedState` NewParam)
      (bind (_scene_component _success_) (message `/Game/Blueprints/BPI/BPI_FoodCooking.GetFoodIngredientMeshes` (`self.ActorRef`)))
      (if _success_
        (for _array_element _scene_component
          (bind _asstatic_mesh_component (cast `StaticMeshComponent` _array_element))
          (bind _returnvalue_2 (`PrimitiveComponent.CreateDynamicMaterialInstance` _asstatic_mesh_component 0 (`PrimitiveComponent.GetMaterial` _asstatic_mesh_component 0) "None"))
          (if (!= (`|GetEnumeratorName` (`self.CookedState`)) (`|GetEnumeratorName` (select `/Game/Blueprints/Enums/E_CookingState` _cookedstate :`NewEnumerator0` "NewEnumerator2" :`NewEnumerator1` "NewEnumerator2" :`NewEnumerator2` "NewEnumerator2" :!type "/Game/Blueprints/Enums/E_CookingState Enum")))
            (bind _returnvalue_3 (`MaterialInstanceDynamic.K2_GetScalarParameterValue` _returnvalue_2 "Cooked_State"))
            (if (!= _returnvalue_3 2.0)
              (`MaterialInstanceDynamic.SetScalarParameterValue` _returnvalue_2 "Cooked_State" (+ _returnvalue_3 1.0)))
            (else
              (`MaterialInstanceDynamic.SetScalarParameterValue` _returnvalue_2 "Cooked_State" (select `/Game/Blueprints/Enums/E_CookingState` _cookedstate :`NewEnumerator1` 1.0 :`NewEnumerator2` 2.0))))))
      ;[1 1 1 0.5 26] Biggest BS of my that I had to fix
      (bind _mesh_component (message `/Game/Blueprints/BPI/BPI_FoodCooking.GetBaseItemMesh` (`self.ActorRef`)))
      (bind _returnvalue_4 (`PrimitiveComponent.CreateDynamicMaterialInstance` _mesh_component 0 (`PrimitiveComponent.GetMaterial` _mesh_component (`self.Base item Material index`)) "None"))
      (`MaterialInstanceDynamic.SetScalarParameterValue` _returnvalue_4 "Cooked_State" _returnvalue)
      (`/Game/Blueprints/BPFL/BPFL_GlobalFunctions.Debug - Print string` (`KismetStringLibrary.Conv_DoubleToString` _returnvalue) false)
      (message `/Game/Blueprints/BPI/BPI_FoodCooking.ActivateSmoke` (`self.ActorRef`))
      (set `self.Heat` (`self.MaxHeat`))
      (`KismetSystemLibrary.K2_SetTimer` null "DecreaseTemperature" 0.5 true))))

(fn `ActivateSmoke`
  (returns (`Success?` :type Boolean))
  (return false))

(fn `GetBaseItemMesh`
  (returns (`Mesh Component` :type "MeshComponent Object Reference"))
  (return null))

(fn `GetFoodIngredientMeshes`
  (returns (`Scene component` :type "Array of SceneComponent Object Reference") (`success?` :type Boolean))
  (return _ false))

(fn `GetWhatOvenCanCook`
  (returns (`WhatOvenType?` :type "/Game/Blueprints/Enums/E_WhatOvenCanCook Enum"))
  (return "NewEnumerator0"))