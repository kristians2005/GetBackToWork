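; BPC_Choping is a component, apparently for chopping, that swaps an item actor for the next stage in a sequence of item classes.
; Init stores the item and builds an ordered class array from its states struct: Before, up to two optional middle stages, then After.
; ChangeItemState runs once, hides the item, spawns the following class at its transform, briefly holds off physics, then destroys the original.
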(event `Init`
  (params (ItemRef :type "/Game/Blueprints/CookingItems/A_BP_BaseItem_Master Object Reference") (ItemStates :type "/Game/Blueprints/DataAssets/ItemState/DA_ItemState Object Reference"))
  (bind _output_get (set `self.Item Ref` ItemRef))
  (bind _output_get_2 (set `self.ItemStates` ItemStates))
  (`/Engine/EditorBlueprintResources/StandardMacros.IsValid` _output_get_2
    (:`Is Valid`
      (set `self.Is Init` true)
      (bind _arr (`self.MakeToArr` (`self.ItemStates`)))
      (set `self.ItemStateArr` _arr))
    (:`Is Not Valid`
      (`/Game/Blueprints/BPFL/BPFL_GlobalFunctions.Debug - Print string` (`KismetTextLibrary.Conv_TextToString` (`|FormatText` "{1} Item state was not selected" _output_get)) true (struct :`R` 1.0 :`B` 0.022033 :`A` 1.0)))))

(event `ChangeItemState`
  (bind _baseitem (`/Game/Blueprints/CookingItems/A_BP_BaseItem_Master.BaseItem` (`self.Item Ref`)))
  (bind (_returnvalue_location _returnvalue_rotation) (`KismetMathLibrary.BreakTransform` (`SceneComponent.K2_GetComponentToWorld` _baseitem)))
  (`/Engine/EditorBlueprintResources/StandardMacros.DoOnce` false
    (:`Completed`
      (for (_array_element _array_index) (`self.ItemStateArr`)
        (if (== _array_element (`GameplayStatics.GetObjectClass` (`self.Item Ref`)))
          (`SceneComponent.SetVisibility` _baseitem false false)
          (bind _returnvalue (`|SpawnActorFromClass` (`|GetArrayItem` (`self.ItemStateArr`) (+ _array_index 1)) (`KismetMathLibrary.MakeTransform` _returnvalue_location _returnvalue_rotation) "Undefined" "MultiplyWithRoot" null true null))
          (`/Game/Blueprints/BPI/BPI_BaseItem.SetSimulatePhisics?` _returnvalue false)
          (`KismetSystemLibrary.Delay` 0.1)
          (`/Game/Blueprints/BPI/BPI_BaseItem.SetSimulatePhisics?` _returnvalue true)
          (`Actor.K2_DestroyActor` (`self.Item Ref`)))))))

(fn `MakeToArr`
  (params (NewParam :type "/Game/Blueprints/DataAssets/ItemState/DA_ItemState Object Reference"))
  (returns (Arr :type "Array of /Game/Blueprints/CookingItems/A_BP_BaseItem_Master Class Reference"))
  (locals (L_arr :type "Array of /Game/Blueprints/CookingItems/A_BP_BaseItem_Master Class Reference"))
  (bind _itemstates (`self.ItemStates`))
  (`KismetArrayLibrary.Array_Add` (`local.L_arr`) (`/Game/Blueprints/DataAssets/ItemState/DA_ItemState.Before` (`self.ItemStates`)))
  (if (`KismetSystemLibrary.IsValidClass` (`/Game/Blueprints/DataAssets/ItemState/DA_ItemState.2` (`self.ItemStates`)))
    (`KismetArrayLibrary.Array_Add` (`local.L_arr`) (`/Game/Blueprints/DataAssets/ItemState/DA_ItemState.2` (`self.ItemStates`))))
  (if (`KismetSystemLibrary.IsValidClass` (`/Game/Blueprints/DataAssets/ItemState/DA_ItemState.3` _itemstates))
    (`KismetArrayLibrary.Array_Add` (`local.L_arr`) (`/Game/Blueprints/DataAssets/ItemState/DA_ItemState.3` (`self.ItemStates`))))
  (`KismetArrayLibrary.Array_Add` (`local.L_arr`) (`/Game/Blueprints/DataAssets/ItemState/DA_ItemState.After` _itemstates))
  (return (`local.L_arr`)))