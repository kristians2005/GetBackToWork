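; Actor component that makes an item cookable, tracking its temperature as it moves from raw to cooked to burnt.
; A looping timer adds heat while cooking, and a slower one cools it after cooking stops.
; Reaching the cooked threshold starts warm smoke, and hitting max heat burns the item.
; State changes go to the item's container component if initialized, otherwise they swap the item's own mesh material.
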(event `Init`
  (params (BaseItem :type "/Game/Blueprints/CookingItems/A_BP_BaseItem_Master Object Reference"))
  (set `self.BaseItemRef` BaseItem))

(event `StartCooking`
  (params (Heat :type "Float (double-precision)"))
  (set `self.Heat` Heat)
  (`KismetSystemLibrary.K2_ClearAndInvalidateTimerHandle` (`self.Decrease Temperature TIme`))
  (`KismetSystemLibrary.K2_SetTimer` null "Increase Temperature" 0.1 true))

(event `StopCooking`
  (`KismetSystemLibrary.K2_ClearTimer` null "Increase Temperature")
  (bind _returnvalue (`KismetSystemLibrary.K2_SetTimer` null "Decrease Temperature" 1.0 true))
  (set `self.Decrease Temperature TIme` _returnvalue))

(event `Increase Temperature`
  (bind _ns_warmsmoke (`/Game/Blueprints/CookingItems/A_BP_BaseItem_Master.NS_WarmSmoke` (`self.BaseItemRef`)))
  (if (< (`self.TemperatureState`) (`self.MaxHeat`))
    (if (< (`self.TemperatureState`) (`self.CookedState`))
      (bind _output_get (set `self.TemperatureState` (+ (`self.Heat`) (`self.TemperatureState`)) :!label _label))
      (`/Game/Blueprints/BPFL/BPFL_GlobalFunctions.Debug - Print string` (`KismetStringLibrary.Conv_DoubleToString` _output_get) false (struct :`R` 0.980146 :`G` 0.936262 :`B` 1.0 :`A` 1.0))
      (elif (`self.IsActive` _ns_warmsmoke)
        (goto _label)
        (else
          (`self.Activate` _ns_warmsmoke true)
          (bind _output_get_2 (set `self.Cooked-state` "NewEnumerator1"))
          (`self.HandleCookedState` _output_get_2))))
    (else
      (bind _output_get_3 (set `self.Cooked-state` "NewEnumerator2"))
      (`self.HandleCookedState` _output_get_3))))

(event `Decrease Temperature`
  (params (heat :type "Float (double-precision)"))
  (bind _output_get (set `self.TemperatureState` (- (`self.TemperatureState`) 5.0)))
  (`/Game/Blueprints/BPFL/BPFL_GlobalFunctions.Debug - Print string` (`KismetStringLibrary.Conv_DoubleToString` _output_get) true (struct :`R` 1.0 :`G` 0.562463 :`A` 1.0) 2.0))

(event `ChangeCookedState`
  (params (enum :type "/Game/Blueprints/Enums/E_CookingState Enum" :default "NewEnumerator0"))
  (bind _item (`/Game/Blueprints/CookingItems/A_BP_BaseItem_Master.Item` (`self.BaseItemRef`)))
  (bind _texture (`/Game/Blueprints/DataAssets/Items/DA_Item.Texture` _item))
  (`/Engine/EditorBlueprintResources/StandardMacros.IsValid` _item
    (:`Is Valid`
      (`/Engine/EditorBlueprintResources/StandardMacros.IsValid` _texture
        (:`Is Valid`
          (`PrimitiveComponent.SetMaterial` (`/Game/Blueprints/CookingItems/A_BP_BaseItem_Master.BaseItem` (`self.BaseItemRef`)) 0 (select `/Game/Blueprints/Enums/E_CookingState` enum :`NewEnumerator0` (`/Game/Blueprints/DataAssets/CookedState/DA_Cooked-state.raw` _texture) :`NewEnumerator1` (`/Game/Blueprints/DataAssets/CookedState/DA_Cooked-state.cooked` _texture) :`NewEnumerator2` (`/Game/Blueprints/DataAssets/CookedState/DA_Cooked-state.burnt` _texture))))))))

(fn `ChangeMeshCookedState`
  (params (Enum_cooked_state :type "/Game/Blueprints/Enums/E_CookingState Enum" :default "NewEnumerator0")))

(fn `HandleCookedState`
  (params (InputPin :type "/Game/Blueprints/Enums/E_CookingState Enum" :default "NewEnumerator0"))
  (if (`/Game/Blueprints/BPC/BPC_Container.Is Initilized?` (`/Game/Blueprints/CookingItems/A_BP_BaseItem_Master.BPC_Container` (`self.BaseItemRef`)))
    (`/Game/Blueprints/BPI/BPI_Container.ChangeMeshCookedState` (`/Game/Blueprints/CookingItems/A_BP_BaseItem_Master.BPC_Container` (`self.BaseItemRef`)) InputPin)
    (else
      (`self.ChangeCookedState` InputPin))))

(fn `TransferContentOutput`
  (returns (NewParam :type "/Game/Blueprints/Structs/ST_Container Structure"))
  (return))